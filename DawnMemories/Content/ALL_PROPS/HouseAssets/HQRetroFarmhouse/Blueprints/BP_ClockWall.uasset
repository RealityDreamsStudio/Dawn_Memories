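; Wall clock prop that rotates hour, minute and second hands to show either the system time or a custom start time.
; Construction script poses the hour and minute hands from Hours and Minutes.
; With ShowRealTime, hands follow Now() every Tick while IsWorking, or are set once at BeginPlay if not.
; Otherwise, a one-second timer, looping only when IsWorking, advances the hands incrementally through CustomTimeUpdate.
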(event Custom|UpdateTime
  (CallFunction|CustomTimeUpdate))

(event EventBeginPlay
  (bind _returnvalue (Math|DateTime|Now))
  (bind _minutes (Variables|ClockProperties|GetMinutes))
  (bind _isworking (Variables|ClockProperties|GetIsWorking))
  (bind _showrealtime (Variables|ClockProperties|GetShowRealTime))
  (bind _returnvalue_2 (Class|KismetMathLibrary|GetSecond _returnvalue))
  (bind _returnvalue_3 (Class|KismetMathLibrary|GetMinute _returnvalue))
  (bind _returnvalue_4 (Math|Conversions|ToFloat(Integer) _returnvalue_2))
  (Utilities|FlowControl|Sequence
    (:then_0
      (if (not _isworking)
        (if _showrealtime
          ;[1 1 1] Real Time
          (Transformation|SetRelativeRotation (Variables|Default|GetSM_ClockWall_Arrow_hours) (Math|Rotator|MakeRotator (* (+ (* (+ (* (Class|KismetMathLibrary|GetHour12 _returnvalue) 6e+01) (Math|Conversions|ToFloat(Integer) _returnvalue_3)) 6e+01) _returnvalue_4) -0.0083333333) 0.0 0.0) false false)
          (Transformation|SetRelativeRotation (Variables|Default|GetSM_ClockWall_Arrow_minutes) (Math|Rotator|MakeRotator (* (+ _returnvalue_4 (* _returnvalue_3 6e+01)) -0.1) 0.0 0.0) false false)
          (Transformation|SetRelativeRotation (Variables|Default|GetSM_ClockWall_Arrow_seconds) (Math|Rotator|MakeRotator (* _returnvalue_2 -6.0) 0.0 0.0) false false))))
    (:then_1
      (if (not _showrealtime)
        (Transformation|SetRelativeRotation (Variables|Default|GetSM_ClockWall_Arrow_minutes) (Math|Rotator|MakeRotator (* _minutes -6.0) 0.0 0.0) false false)
        (Transformation|SetRelativeRotation (Variables|Default|GetSM_ClockWall_Arrow_hours) (Math|Rotator|MakeRotator (+ (* _minutes -0.5) (* (Variables|ClockProperties|GetHours) -3e+01)) 0.0 0.0) false false)
        (Utilities|Time|SetTimerbyEvent (delegate Custom|UpdateTime) 1.0 _isworking)))))

(event EventTick
  (params (DeltaSeconds :type Float%20%28single-precision%29))
  (bind _returnvalue (Math|DateTime|Now))
  (bind _returnvalue_2 (Class|KismetMathLibrary|GetSecond _returnvalue))
  (bind _returnvalue_3 (Class|KismetMathLibrary|GetMinute _returnvalue))
  (bind _returnvalue_4 (Math|Conversions|ToFloat(Integer) _returnvalue_2))
  (if (Variables|ClockProperties|GetIsWorking)
    (if (Variables|ClockProperties|GetShowRealTime)
      ;[1 1 1] Real Time
      (Transformation|SetRelativeRotation (Variables|Default|GetSM_ClockWall_Arrow_hours) (Math|Rotator|MakeRotator (* (+ (* (+ (* (Class|KismetMathLibrary|GetHour12 _returnvalue) 6e+01) (Math|Conversions|ToFloat(Integer) _returnvalue_3)) 6e+01) _returnvalue_4) -0.0083333333) 0.0 0.0) false false)
      (Transformation|SetRelativeRotation (Variables|Default|GetSM_ClockWall_Arrow_minutes) (Math|Rotator|MakeRotator (* (+ _returnvalue_4 (* _returnvalue_3 6e+01)) -0.1) 0.0 0.0) false false)
      (Transformation|SetRelativeRotation (Variables|Default|GetSM_ClockWall_Arrow_seconds) (Math|Rotator|MakeRotator (* _returnvalue_2 -6.0) 0.0 0.0) false false))))

(fn ConstructionScript
  (bind _minutes (Variables|ClockProperties|GetMinutes))
  (Transformation|SetRelativeRotation (Variables|Default|GetSM_ClockWall_Arrow_minutes) (Math|Rotator|MakeRotator (* _minutes -6.0) 0.0 0.0) false false)
  (Transformation|SetRelativeRotation (Variables|Default|GetSM_ClockWall_Arrow_hours) (Math|Rotator|MakeRotator (+ (* _minutes -0.5) (* (Variables|ClockProperties|GetHours) -3e+01)) 0.0 0.0) false false))

(fn CustomTimeUpdate
  (Transformation|AddLocalRotation (Variables|Default|GetSM_ClockWall_Arrow_seconds) (Math|Rotator|MakeRotator -6.0 0.0 0.0) false false)
  (Transformation|AddLocalRotation (Variables|Default|GetSM_ClockWall_Arrow_minutes) (Math|Rotator|MakeRotator -0.1 0.0 0.0) false false)
  (Transformation|AddLocalRotation (Variables|Default|GetSM_ClockWall_Arrow_hours) (Math|Rotator|MakeRotator -0.008333333 0.0 0.0) false false))