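; BP_CeilingLamp_A is a configurable ceiling lamp prop for the retro farmhouse assets, set up entirely in the construction script.
; It applies per-slot material overrides to the lamp mesh and writes the resulting material list back to MaterialsOverride.
; The Light flag controls whether the spotlight is destroyed and the emissive zeroed.
; Shared intensity and color values drive both the spotlight and a dynamic material instance on slot 0, keeping glow and light matched.
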(event EventBeginPlay)

(event Collision|EventActorBeginOverlap
  (params (OtherActor :type Actor%20Object%20Reference)))

(event EventTick
  (params (DeltaSeconds :type Float%20%28single-precision%29)))

(fn ConstructionScript
  (bind _light (Variables|LampProperties|GetLight))
  (bind _light_color (Variables|LampProperties|GetLight%20Color))
  (bind _sm_ceilinglamp_a (Variables|Default|GetSM_CeilingLamp_A))
  (bind _light_intensity (Variables|LampProperties|GetLight%20Intensity))
  (bind _spotlight (Variables|Default|GetSpotLight))
  (bind _initmaterials (CallFunction|OverrideMeshMaterials _sm_ceilinglamp_a (Variables|Materials|GetMaterials%20Override)))
  (Variables|Materials|SetMaterials%20Override _initmaterials)
  (if _light
    _
    (else
      (Components|DestroyComponent _spotlight)))
  (CallFunction|LightProperties _spotlight _light_intensity _light_color)
  (CallFunction|MaterialProperties _sm_ceilinglamp_a _light_intensity _light_color _light))

(fn LightProperties
  (params (Light%20Component :type Light%20Component%20Object%20Reference) (Light%20Intensity :type Float%20%28single-precision%29) (Light%20Color :type Color%20Structure))
  (Rendering|Components|Light|SetIntensity Light%20Component Light%20Intensity)
  (Rendering|Components|Light|SetLightColor Light%20Component (Math|Conversions|ToLinearColor(Color) Light%20Color) true))

(fn MaterialProperties
  (params (Mesh :type Static%20Mesh%20Component%20Object%20Reference) (Light%20Intensity :type Float%20%28single-precision%29) (Light%20Color :type Color%20Structure) (isLight :type Boolean))
  (bind _returnvalue (Rendering|Material|CreateDynamicMaterialInstance Mesh 0 (Rendering|Material|GetMaterial Mesh 0) "None" :!class /Script/Engine.PrimitiveComponent))
  (Rendering|Material|SetScalarParameterValue _returnvalue "Emissive Intensity" (select isLight (* Light%20Intensity 0.0085) 0.0) :!class /Script/Engine.MaterialInstanceDynamic)
  (Rendering|Material|SetVectorParameterValue _returnvalue "Emissive Color" (Math|Conversions|ToLinearColor(Color) Light%20Color) :!class /Script/Engine.MaterialInstanceDynamic))

(fn OverrideMeshMaterials
  (params (Mesh :type Static%20Mesh%20Component%20Object%20Reference) (Materials :type Array%20of%20Material%20Interface%20Object%20References))
  (bind _returnvalue (Rendering|Material|GetMaterials Mesh))
  (for (_ _array_index) _returnvalue
    (Utilities|Array|Resize Materials (Rendering|Material|GetNumMaterials Mesh))
    (Rendering|Material|SetMaterial Mesh _array_index (Utilities|Array|Get(acopy) Materials _array_index)))
  (return _returnvalue))