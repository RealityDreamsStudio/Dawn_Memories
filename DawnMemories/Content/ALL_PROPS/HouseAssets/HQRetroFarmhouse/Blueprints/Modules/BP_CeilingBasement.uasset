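; Modular basement ceiling piece for the retro farmhouse house kit, built entirely in the construction script.
; A ModuleType enum selects one of five static mesh components to add.
; A helper resizes the MaterialsOverride array to the mesh's slot count, applies each entry, then writes the mesh's resulting materials back into that array.
; The event graph holds no active logic.
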(event EventBeginPlay)

(event Collision|EventActorBeginOverlap
  (params (OtherActor :type Actor%20Object%20Reference)))

(event EventTick
  (params (DeltaSeconds :type Float%20%28single-precision%29)))

(fn ConstructionScript
  (switch Utilities|FlowControl|Switch|Switchon (Variables|ModuleProperties|GetModule%20Type)
    (:NewEnumerator0
      (bind _returnvalue (AddComponent|AddStaticMeshComponent false))
      (bind _initmaterials (CallFunction|OverrideMeshMaterials _returnvalue (Variables|Materials|GetMaterials%20Override)))
      (Variables|Materials|SetMaterials%20Override _initmaterials))
    (:NewEnumerator1
      (bind _returnvalue_2 (AddComponent|AddStaticMeshComponent false))
      (bind _initmaterials_2 (CallFunction|OverrideMeshMaterials _returnvalue_2 (Variables|Materials|GetMaterials%20Override)))
      (Variables|Materials|SetMaterials%20Override _initmaterials_2))
    (:NewEnumerator2
      (bind _returnvalue_3 (AddComponent|AddStaticMeshComponent false))
      (bind _initmaterials_3 (CallFunction|OverrideMeshMaterials _returnvalue_3 (Variables|Materials|GetMaterials%20Override)))
      (Variables|Materials|SetMaterials%20Override _initmaterials_3))
    (:NewEnumerator3
      (bind _returnvalue_4 (AddComponent|AddStaticMeshComponent false))
      (bind _initmaterials_4 (CallFunction|OverrideMeshMaterials _returnvalue_4 (Variables|Materials|GetMaterials%20Override)))
      (Variables|Materials|SetMaterials%20Override _initmaterials_4))
    (:NewEnumerator4
      (bind _returnvalue_5 (AddComponent|AddStaticMeshComponent false))
      (bind _initmaterials_5 (CallFunction|OverrideMeshMaterials _returnvalue_5 (Variables|Materials|GetMaterials%20Override)))
      (Variables|Materials|SetMaterials%20Override _initmaterials_5))))

(fn OverrideMeshMaterials
  (params (Mesh :type Static%20Mesh%20Component%20Object%20Reference) (Materials :type Array%20of%20Material%20Interface%20Object%20References))
  (bind _returnvalue (Rendering|Material|GetMaterials Mesh))
  (for (_ _array_index) _returnvalue
    (Utilities|Array|Resize Materials (Rendering|Material|GetNumMaterials Mesh))
    (Rendering|Material|SetMaterial Mesh _array_index (Utilities|Array|Get(acopy) Materials _array_index)))
  (return _returnvalue))