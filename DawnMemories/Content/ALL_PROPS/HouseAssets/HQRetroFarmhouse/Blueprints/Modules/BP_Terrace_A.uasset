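; Modular terrace piece for the retro farmhouse kit, assembled entirely in the construction script.
; ModuleType selects one of seven variants and the Broken flag picks between two versions of each, adding the matching static mesh component.
; OverrideMeshMaterials resizes MaterialsOverride to the mesh's slot count, applies it per slot, and the mesh's resulting materials are written back into that array.
; The event graph holds only disabled stub events.
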(event EventBeginPlay)

(event Collision|EventActorBeginOverlap
  (params (OtherActor :type Actor%20Object%20Reference)))

(event EventTick
  (params (DeltaSeconds :type Float%20%28single-precision%29)))

(fn ConstructionScript
  (bind _broken (Variables|ModuleProperties|GetBroken))
  (switch Utilities|FlowControl|Switch|Switchon (Variables|ModuleProperties|GetModule%20Type)
    (:NewEnumerator0
      (if _broken
        (bind _returnvalue (AddComponent|AddStaticMeshComponent false))
        (bind _initmaterials (CallFunction|OverrideMeshMaterials _returnvalue (Variables|ModuleMaterials|GetMaterialsOverride)))
        (Variables|ModuleMaterials|SetMaterialsOverride _initmaterials)
        (else
          (bind _returnvalue_2 (AddComponent|AddStaticMeshComponent false))
          (bind _initmaterials_2 (CallFunction|OverrideMeshMaterials _returnvalue_2 (Variables|ModuleMaterials|GetMaterialsOverride)))
          (Variables|ModuleMaterials|SetMaterialsOverride _initmaterials_2))))
    (:NewEnumerator3
      (if _broken
        (bind _returnvalue_3 (AddComponent|AddStaticMeshComponent false))
        (bind _initmaterials_3 (CallFunction|OverrideMeshMaterials _returnvalue_3 (Variables|ModuleMaterials|GetMaterialsOverride)))
        (Variables|ModuleMaterials|SetMaterialsOverride _initmaterials_3)
        (else
          (bind _returnvalue_4 (AddComponent|AddStaticMeshComponent false))
          (bind _initmaterials_4 (CallFunction|OverrideMeshMaterials _returnvalue_4 (Variables|ModuleMaterials|GetMaterialsOverride)))
          (Variables|ModuleMaterials|SetMaterialsOverride _initmaterials_4))))
    (:NewEnumerator4
      (if _broken
        (bind _returnvalue_5 (AddComponent|AddStaticMeshComponent false))
        (bind _initmaterials_5 (CallFunction|OverrideMeshMaterials _returnvalue_5 (Variables|ModuleMaterials|GetMaterialsOverride)))
        (Variables|ModuleMaterials|SetMaterialsOverride _initmaterials_5)
        (else
          (bind _returnvalue_6 (AddComponent|AddStaticMeshComponent false))
          (bind _initmaterials_6 (CallFunction|OverrideMeshMaterials _returnvalue_6 (Variables|ModuleMaterials|GetMaterialsOverride)))
          (Variables|ModuleMaterials|SetMaterialsOverride _initmaterials_6))))
    (:NewEnumerator15
      (if _broken
        (bind _returnvalue_7 (AddComponent|AddStaticMeshComponent false))
        (bind _initmaterials_7 (CallFunction|OverrideMeshMaterials _returnvalue_7 (Variables|ModuleMaterials|GetMaterialsOverride)))
        (Variables|ModuleMaterials|SetMaterialsOverride _initmaterials_7)
        (else
          (bind _returnvalue_8 (AddComponent|AddStaticMeshComponent false))
          (bind _initmaterials_8 (CallFunction|OverrideMeshMaterials _returnvalue_8 (Variables|ModuleMaterials|GetMaterialsOverride)))
          (Variables|ModuleMaterials|SetMaterialsOverride _initmaterials_8))))
    (:NewEnumerator5
      (if _broken
        (bind _returnvalue_9 (AddComponent|AddStaticMeshComponent false))
        (bind _initmaterials_9 (CallFunction|OverrideMeshMaterials _returnvalue_9 (Variables|ModuleMaterials|GetMaterialsOverride)))
        (Variables|ModuleMaterials|SetMaterialsOverride _initmaterials_9)
        (else
          (bind _returnvalue_10 (AddComponent|AddStaticMeshComponent false))
          (bind _initmaterials_10 (CallFunction|OverrideMeshMaterials _returnvalue_10 (Variables|ModuleMaterials|GetMaterialsOverride)))
          (Variables|ModuleMaterials|SetMaterialsOverride _initmaterials_10))))
    (:NewEnumerator13
      (if _broken
        (bind _returnvalue_11 (AddComponent|AddStaticMeshComponent false))
        (bind _initmaterials_11 (CallFunction|OverrideMeshMaterials _returnvalue_11 (Variables|ModuleMaterials|GetMaterialsOverride)))
        (Variables|ModuleMaterials|SetMaterialsOverride _initmaterials_11)
        (else
          (bind _returnvalue_12 (AddComponent|AddStaticMeshComponent false))
          (bind _initmaterials_12 (CallFunction|OverrideMeshMaterials _returnvalue_12 (Variables|ModuleMaterials|GetMaterialsOverride)))
          (Variables|ModuleMaterials|SetMaterialsOverride _initmaterials_12))))
    (:NewEnumerator14
      (if _broken
        (bind _returnvalue_13 (AddComponent|AddStaticMeshComponent false))
        (bind _initmaterials_13 (CallFunction|OverrideMeshMaterials _returnvalue_13 (Variables|ModuleMaterials|GetMaterialsOverride)))
        (Variables|ModuleMaterials|SetMaterialsOverride _initmaterials_13)
        (else
          (bind _returnvalue_14 (AddComponent|AddStaticMeshComponent false))
          (bind _initmaterials_14 (CallFunction|OverrideMeshMaterials _returnvalue_14 (Variables|ModuleMaterials|GetMaterialsOverride)))
          (Variables|ModuleMaterials|SetMaterialsOverride _initmaterials_14))))))

(fn OverrideMeshMaterials
  (params (Mesh :type Static%20Mesh%20Component%20Object%20Reference) (Materials :type Array%20of%20Material%20Interface%20Object%20References))
  (bind _returnvalue (Rendering|Material|GetMaterials Mesh))
  (for (_ _array_index) _returnvalue
    (Utilities|Array|Resize Materials (Rendering|Material|GetNumMaterials Mesh))
    (Rendering|Material|SetMaterial Mesh _array_index (Utilities|Array|Get(acopy) Materials _array_index)))
  (return _returnvalue))