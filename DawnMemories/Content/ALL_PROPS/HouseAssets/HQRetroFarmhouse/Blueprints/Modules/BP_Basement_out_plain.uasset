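; Modular farmhouse basement exterior piece, assembled in the Construction Script with no runtime logic.
; ModuleType selects a blank wall, window, bay or patch mesh, with an optional rotated interior mesh.
; Windows() acts only on the window type, adding a child-actor window plus optional emissive light mesh via dynamic material and Lightmass portal.
; Helpers apply per-slot material overrides, writing mesh materials back into exterior and interior override arrays.
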(event EventBeginPlay)

(event Collision|EventActorBeginOverlap
  (params (OtherActor :type Actor%20Object%20Reference)))

(event EventTick
  (params (DeltaSeconds :type Float%20%28single-precision%29)))

(fn ConstructionScript
  (bind _returnvalue (Math|Transform|MakeTransform "0.000000,-250.000000,0.000000" "0,180.000000, 0"))
  (switch Utilities|FlowControl|Switch|Switchon (Variables|ModuleProperties|GetModule%20Type)
    (:NewEnumerator0
      ;[1 1 1] Blank wall
      (bind _returnvalue_2 (AddComponent|AddStaticMeshComponent false))
      (bind _initmaterials (CallFunction|OverrideMeshMaterials _returnvalue_2 (Variables|ModuleMaterials|GetExteriorMaterialsOverride)))
      (Variables|ModuleMaterials|SetExteriorMaterialsOverride _initmaterials)
      ;;[1 1 1] Interior
      (if (Variables|ModuleProperties|GetInterior)
        (bind _returnvalue_3 (AddComponent|AddStaticMeshComponent false _returnvalue))
        (Variables|Default|SetInteriorMesh _returnvalue_3)))
    (:NewEnumerator3
      ;[1 1 1] Window
      (bind _returnvalue_4 (AddComponent|AddStaticMeshComponent false))
      (bind _initmaterials_2 (CallFunction|OverrideMeshMaterials _returnvalue_4 (Variables|ModuleMaterials|GetExteriorMaterialsOverride)))
      (Variables|ModuleMaterials|SetExteriorMaterialsOverride _initmaterials_2)
      ;;[1 1 1] Interior
      (if (Variables|ModuleProperties|GetInterior)
        (bind _returnvalue_5 (AddComponent|AddStaticMeshComponent false _returnvalue))
        (Variables|Default|SetInteriorMesh _returnvalue_5))
      (if (Variables|ModuleProperties|GetWindow) :!label _label
        (CallFunction|Windows)))
    (:NewEnumerator4
      ;[1 1 1] Bay
      (bind _returnvalue_6 (AddComponent|AddStaticMeshComponent false))
      (bind _initmaterials_3 (CallFunction|OverrideMeshMaterials _returnvalue_6 (Variables|ModuleMaterials|GetExteriorMaterialsOverride)))
      (Variables|ModuleMaterials|SetExteriorMaterialsOverride _initmaterials_3)
      ;;[1 1 1] Interior
      (if (Variables|ModuleProperties|GetInterior)
        (bind _returnvalue_7 (AddComponent|AddStaticMeshComponent false _returnvalue))
        (Variables|Default|SetInteriorMesh _returnvalue_7)
        (goto _label)
        (else
          (goto _label))))
    (:NewEnumerator5
      ;[1 1 1] Patch
      (bind _returnvalue_8 (AddComponent|AddStaticMeshComponent false))
      (bind _initmaterials_4 (CallFunction|OverrideMeshMaterials _returnvalue_8 (Variables|ModuleMaterials|GetExteriorMaterialsOverride)))
      (Variables|ModuleMaterials|SetExteriorMaterialsOverride _initmaterials_4)
      ;;[1 1 1] Interior
      (if (Variables|ModuleProperties|GetInterior)
        (bind _returnvalue_9 (AddComponent|AddStaticMeshComponent false (Math|Transform|MakeTransform "0.000000,-50.000000,0.000000" "0,180.000000, 0")))
        (Variables|Default|SetInteriorMesh _returnvalue_9)
        (goto _label)
        (else
          (goto _label)))))
  (bind _initmaterials_5 (CallFunction|OverrideMeshMaterials (Variables|Default|GetInteriorMesh) (Variables|ModuleMaterials|GetInteriorMaterialsOverride)))
  (Variables|ModuleMaterials|SetInteriorMaterialsOverride _initmaterials_5))

(fn Windows
  (bind _returnvalue (Math|Transform|MakeTransform "-18.000000,-125.000000,28.500000"))
  (switch Utilities|FlowControl|Switch|Switchon (Variables|ModuleProperties|GetModule%20Type)
    (:NewEnumerator3
      (bind _returnvalue_2 (AddComponent|AddChildActorComponent false _returnvalue))
      (CallFunction|OverrideChildActorMaterials _returnvalue_2 (Variables|Default|GetWindowStaticMeshes) (Variables|Default|GetWindowMaterials) (Variables|ModuleMaterials|GetWindowMaterialsOverride))
      (if (Variables|WindowLight|GetWindow%20Light)
        (bind _returnvalue_3 (AddComponent|AddStaticMeshComponent false _returnvalue))
        (CallFunction|SetWindowLightMaterialProperties _returnvalue_3 (Variables|WindowLight|GetWindow%20Light%20Intensity) (Variables|WindowLight|GetWindow%20Light%20Color)))
      (if (Variables|WindowLight|GetLightmass%20Portal)
        (AddComponent|AddChildActorComponent false (Math|Transform|MakeTransform "-20.000000,-125.000000,28.000000" "0, 0, 0" "1.000000,0.250000,0.150000"))))))

(fn OverrideMeshMaterials
  (params (Mesh :type Static%20Mesh%20Component%20Object%20Reference) (Materials :type Array%20of%20Material%20Interface%20Object%20References))
  (bind _returnvalue (Rendering|Material|GetMaterials Mesh))
  (for (_ _array_index) _returnvalue
    (Utilities|Array|Resize Materials (Rendering|Material|GetNumMaterials Mesh))
    (Rendering|Material|SetMaterial Mesh _array_index (Utilities|Array|Get(acopy) Materials _array_index)))
  (return _returnvalue))

(fn OverrideChildActorMaterials
  (params (ChildActor :type Child%20Actor%20Component%20Object%20Reference) (StaticMeshes :type Array%20of%20Static%20Mesh%20Component%20Object%20References) (MeshesMaterials :type Array%20of%20Material%20Interface%20Object%20References) (MaterialOverrides :type Array%20of%20Material%20Interface%20Object%20References))
  (for _array_element (Components|GetChildrenComponents ChildActor true)
    (bind _asstatic_mesh_component (Utilities|Casting|CastToStaticMeshComponent _array_element))
    (Utilities|Array|Add StaticMeshes _asstatic_mesh_component))
  (for _array_element_2 StaticMeshes
    (Utilities|Array|Add MeshesMaterials (Rendering|Material|GetMaterial _array_element_2 0)))
  (for (_array_element_3 _array_index) StaticMeshes
    (Rendering|Material|SetMaterial _array_element_3 0 (Utilities|Array|Get(acopy) MaterialOverrides _array_index)))
  (Utilities|Array|Resize MaterialOverrides (Utilities|Array|Length MeshesMaterials)))

(fn SetWindowLightMaterialProperties
  (params (Mesh :type Static%20Mesh%20Component%20Object%20Reference) (Light%20Intensity :type Float%20%28single-precision%29) (Light%20Color :type Color%20Structure))
  (bind _returnvalue (Rendering|Material|CreateDynamicMaterialInstance Mesh 0 (Rendering|Material|GetMaterial Mesh 0) "None" :!class /Script/Engine.PrimitiveComponent))
  (Rendering|Material|SetScalarParameterValue _returnvalue "Emissive Intensity" Light%20Intensity :!class /Script/Engine.MaterialInstanceDynamic)
  (Rendering|Material|SetVectorParameterValue _returnvalue "Emissive Color" (Math|Conversions|ToLinearColor(Color) Light%20Color) :!class /Script/Engine.MaterialInstanceDynamic))