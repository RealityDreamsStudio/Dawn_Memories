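; BP_Roof is a modular roof piece for the retro farmhouse kit, assembled entirely in the Construction Script.
; ModuleType selects the roof mesh component to add.
; When Gutter is on, AddGutters adds a mirrored pair for most module types, with a BrokenGutter variant.
; Helper functions apply the roof and gutter material override arrays, resizing them to slot count and writing the resulting materials back.
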(event EventBeginPlay)

(event Collision|EventActorBeginOverlap
  (params (OtherActor :type Actor%20Object%20Reference)))

(event EventTick
  (params (DeltaSeconds :type Float%20%28single-precision%29)))

(fn ConstructionScript
  (switch Utilities|FlowControl|Switch|Switchon (Variables|ModuleProperties|GetModule%20Type)
    (:NewEnumerator0
      (bind _returnvalue (AddComponent|AddStaticMeshComponent false))
      (bind _initmaterials (CallFunction|OverrideMeshMaterials _returnvalue (Variables|ModuleMaterials|GetRoofMaterialsOverride)))
      (Variables|ModuleMaterials|SetRoofMaterialsOverride _initmaterials))
    (:NewEnumerator1
      (bind _returnvalue_2 (AddComponent|AddStaticMeshComponent false))
      (bind _initmaterials_2 (CallFunction|OverrideMeshMaterials _returnvalue_2 (Variables|ModuleMaterials|GetRoofMaterialsOverride)))
      (Variables|ModuleMaterials|SetRoofMaterialsOverride _initmaterials_2))
    (:NewEnumerator2
      (bind _returnvalue_3 (AddComponent|AddStaticMeshComponent false))
      (bind _initmaterials_3 (CallFunction|OverrideMeshMaterials _returnvalue_3 (Variables|ModuleMaterials|GetRoofMaterialsOverride)))
      (Variables|ModuleMaterials|SetRoofMaterialsOverride _initmaterials_3))
    (:NewEnumerator3
      (bind _returnvalue_4 (AddComponent|AddStaticMeshComponent false))
      (bind _initmaterials_4 (CallFunction|OverrideMeshMaterials _returnvalue_4 (Variables|ModuleMaterials|GetRoofMaterialsOverride)))
      (Variables|ModuleMaterials|SetRoofMaterialsOverride _initmaterials_4))
    (:NewEnumerator4
      (bind _returnvalue_5 (AddComponent|AddStaticMeshComponent false))
      (bind _initmaterials_5 (CallFunction|OverrideMeshMaterials _returnvalue_5 (Variables|ModuleMaterials|GetRoofMaterialsOverride)))
      (Variables|ModuleMaterials|SetRoofMaterialsOverride _initmaterials_5))
    (:NewEnumerator5
      (bind _returnvalue_6 (AddComponent|AddStaticMeshComponent false))
      (bind _initmaterials_6 (CallFunction|OverrideMeshMaterials _returnvalue_6 (Variables|ModuleMaterials|GetRoofMaterialsOverride)))
      (Variables|ModuleMaterials|SetRoofMaterialsOverride _initmaterials_6))
    (:NewEnumerator6
      (bind _returnvalue_7 (AddComponent|AddStaticMeshComponent false))
      (bind _initmaterials_7 (CallFunction|OverrideMeshMaterials _returnvalue_7 (Variables|ModuleMaterials|GetRoofMaterialsOverride)))
      (Variables|ModuleMaterials|SetRoofMaterialsOverride _initmaterials_7))
    (:NewEnumerator7
      (bind _returnvalue_8 (AddComponent|AddStaticMeshComponent false))
      (bind _initmaterials_8 (CallFunction|OverrideMeshMaterials _returnvalue_8 (Variables|ModuleMaterials|GetRoofMaterialsOverride)))
      (Variables|ModuleMaterials|SetRoofMaterialsOverride _initmaterials_8))
    (:NewEnumerator8
      (bind _returnvalue_9 (AddComponent|AddStaticMeshComponent false))
      (bind _initmaterials_9 (CallFunction|OverrideMeshMaterials _returnvalue_9 (Variables|ModuleMaterials|GetRoofMaterialsOverride)))
      (Variables|ModuleMaterials|SetRoofMaterialsOverride _initmaterials_9))
    (:NewEnumerator9
      (bind _returnvalue_10 (AddComponent|AddStaticMeshComponent false))
      (bind _initmaterials_10 (CallFunction|OverrideMeshMaterials _returnvalue_10 (Variables|ModuleMaterials|GetRoofMaterialsOverride)))
      (Variables|ModuleMaterials|SetRoofMaterialsOverride _initmaterials_10))
    (:NewEnumerator11
      (bind _returnvalue_11 (AddComponent|AddStaticMeshComponent false))
      (bind _initmaterials_11 (CallFunction|OverrideMeshMaterials _returnvalue_11 (Variables|ModuleMaterials|GetRoofMaterialsOverride)))
      (Variables|ModuleMaterials|SetRoofMaterialsOverride _initmaterials_11))
    (:NewEnumerator12
      (bind _returnvalue_12 (AddComponent|AddStaticMeshComponent false))
      (bind _initmaterials_12 (CallFunction|OverrideMeshMaterials _returnvalue_12 (Variables|ModuleMaterials|GetRoofMaterialsOverride)))
      (Variables|ModuleMaterials|SetRoofMaterialsOverride _initmaterials_12)))
  (bind _meshes (CallFunction|AddGutters))
  (bind _initmaterials_13 (CallFunction|OverrideMeshesMaterials _meshes (Variables|ModuleMaterials|GetGutterMaterialsOverride)))
  (Variables|ModuleMaterials|SetGutterMaterialsOverride _initmaterials_13))

(fn OverrideMeshMaterials
  (params (Mesh :type Static%20Mesh%20Component%20Object%20Reference) (Materials :type Array%20of%20Material%20Interface%20Object%20References))
  (bind _returnvalue (Rendering|Material|GetMaterials Mesh))
  (for (_ _array_index) _returnvalue
    (Utilities|Array|Resize Materials (Rendering|Material|GetNumMaterials Mesh))
    (Rendering|Material|SetMaterial Mesh _array_index (Utilities|Array|Get(acopy) Materials _array_index)))
  (return _returnvalue))

(fn AddGutters
  (bind _gutterstaticmeshes (Variables|Default|GetGutterStaticMeshes))
  (bind _module_type (Variables|ModuleProperties|GetModule%20Type))
  (bind _gutterstaticmeshes_2 (Variables|Default|GetGutterStaticMeshes))
  (bind _returnvalue (Utilities|Select :Index _module_type :Option%200 "0, 0, 0" :Option%201 "0, 0, 0" :Option%202 "0, 0, 0" :Option%203 "0, 0, 0" :Option%204 "0, 0, 0" :Option%205 "0, 0, 0" :Option%206 "0, 0, 0" :Option%207 "0, 0, 0" :Option%208 "0, 0, 0" :Option%209 "0, 0, 0" :Option%2010 "0, 0, 0" :Option%2011 "0, 0, 0"))
  (bind _returnvalue_2 (Utilities|Select :Index _module_type :Option%200 "0, 0, 0" :Option%201 "0, 0, 0" :Option%202 "0, 0, 0" :Option%203 "0, 0, 0" :Option%204 "0, 0, 0" :Option%205 "0, 0, 0" :Option%206 "0, 0, 0" :Option%207 "0, 0, 0" :Option%208 "0, 0, 0" :Option%209 "0, 0, 0" :Option%2010 "0, 0, 0" :Option%2011 "0, 0, 0"))
  (bind _returnvalue_3 (Math|Transform|MakeTransform _returnvalue "0,90.000000, 0" "1,-1.000000,1"))
  (bind _returnvalue_4 (Math|Transform|MakeTransform _returnvalue_2 "0,-90.000000, 0"))
  (if (Variables|ModuleProperties|GetGutter)
    (switch Utilities|FlowControl|Switch|Switchon _module_type
      (:NewEnumerator0
        ;[1 1 1] Gutters End
        (if (Variables|ModuleProperties|GetBrokenGutter) :!label _label
          (bind _returnvalue_5 (AddComponent|AddStaticMeshComponent false _returnvalue_4))
          (Utilities|Array|Add _gutterstaticmeshes _returnvalue_5)
          (bind _returnvalue_6 (AddComponent|AddStaticMeshComponent false _returnvalue_3))
          (Utilities|Array|Add _gutterstaticmeshes _returnvalue_6)
          (else
            (bind _returnvalue_7 (AddComponent|AddStaticMeshComponent false _returnvalue_4))
            (Utilities|Array|Add _gutterstaticmeshes _returnvalue_7)
            (bind _returnvalue_8 (AddComponent|AddStaticMeshComponent false _returnvalue_3))
            (Utilities|Array|Add _gutterstaticmeshes _returnvalue_8))))
      (:NewEnumerator1
        ;[1 1 1] Gutters End
        (if (Variables|ModuleProperties|GetBrokenGutter) :!label _label_2
          (bind _returnvalue_9 (AddComponent|AddStaticMeshComponent false _returnvalue_4))
          (Utilities|Array|Add _gutterstaticmeshes_2 _returnvalue_9)
          (bind _returnvalue_10 (AddComponent|AddStaticMeshComponent false _returnvalue_3))
          (Utilities|Array|Add _gutterstaticmeshes_2 _returnvalue_10)
          (else
            (bind _returnvalue_11 (AddComponent|AddStaticMeshComponent false _returnvalue_4))
            (Utilities|Array|Add _gutterstaticmeshes_2 _returnvalue_11)
            (bind _returnvalue_12 (AddComponent|AddStaticMeshComponent false _returnvalue_3))
            (Utilities|Array|Add _gutterstaticmeshes_2 _returnvalue_12))))
      (:NewEnumerator2
        (goto _label))
      (:NewEnumerator3
        (goto _label_2))
      (:NewEnumerator4
        (goto _label))
      (:NewEnumerator5
        (goto _label_2))
      (:NewEnumerator6
        (goto _label))
      (:NewEnumerator7
        (goto _label_2))
      (:NewEnumerator8
        (goto _label))
      (:NewEnumerator9
        (goto _label_2)))
    (return (Variables|Default|GetGutterStaticMeshes))))

(fn OverrideMeshesMaterials
  (params (Mesh :type Array%20of%20Static%20Mesh%20Component%20Object%20References) (Materials :type Array%20of%20Material%20Interface%20Object%20References))
  (for _array_element Mesh
    (for (_ _array_index) (Rendering|Material|GetMaterials _array_element)
      (Utilities|Array|Resize Materials (Rendering|Material|GetNumMaterials _array_element))
      (for _array_element_2 Mesh
        (Rendering|Material|SetMaterial _array_element_2 _array_index (Utilities|Array|Get(acopy) Materials _array_index))))
    (return (Rendering|Material|GetMaterials _array_element))))