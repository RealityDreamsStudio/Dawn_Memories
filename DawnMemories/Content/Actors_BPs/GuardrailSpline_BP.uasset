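; Guardrail actor that builds a mesh along an editable spline in the Construction Script.
; For each pair of consecutive spline points it adds a Spline Mesh Component with the configured mesh, forward axis, collision and character step-up setting.
; Each segment takes local positions and end tangent from its own points, but every start tangent comes from point 0.
; The event graph is unused.
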(event EventBeginPlay)

(event Collision|EventActorBeginOverlap
  (params (OtherActor :type Actor%20Object%20Reference)))

(event EventTick
  (params (DeltaSeconds :type Float%20%28single-precision%29)))

(fn ConstructionScript
  (bind _spline (Variables|Default|GetSpline))
  (bind _spline_2 (Variables|Default|GetSpline))
  (for _index (range 0 (- (Spline|GetNumberOfSplinePoints (Variables|Default|GetSpline)) 2))
    (bind _returnvalue (AddComponent|AddSplineMeshComponent false))
    (Components|StaticMesh|SetStaticMesh _returnvalue (Variables|Default|GetStaticMesh))
    (SplineMesh|SetForwardAxis _returnvalue (Variables|Default|GetIn%20Forward%20Axis) true)
    (Collision|SetCollisionEnabled _returnvalue (Variables|Default|GetNew%20Type))
    (Variables|/Script/Engine.PrimitiveComponent|SetCanCharacterStepUpOn _returnvalue (Variables|Default|GetCan%20Character%20Step%20Up%20On))
    (SplineMesh|SetStartandEnd _returnvalue (Spline|GetLocationatSplinePoint _spline _index "Local") (Spline|GetTangentatSplinePoint _spline 0 "Local") (Spline|GetLocationatSplinePoint _spline_2 (+ _index 1) "Local") (Spline|GetTangentatSplinePoint _spline_2 (+ _index 1) "Local") true :!class /Script/Engine.SplineMeshComponent)))