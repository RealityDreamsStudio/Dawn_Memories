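; Interactable drawer that, when CanOpen is set, plays a one-time camera sequence of sliding open and flags Collectible_BP_Drawer as revealed.
; Two overlap spheres switch between indicator and input prompt, with the inner one enabling Interact.
; During the sequence, player input is disabled and Tick runs a flickering point light.
; AddToPin unlocks it on a matching PIN, but the keypad-creation, line-trace and timeline slide logic is disconnected.
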(event OnComponentBeginOverlap(BiggerSphere)
  (params (OverlappedComponent :type Primitive%20Component%20Object%20Reference) (OtherActor :type Actor%20Object%20Reference) (OtherComp :type Primitive%20Component%20Object%20Reference) (OtherBodyIndex :type Integer) (bFromSweep :type Boolean) (SweepResult :type Hit%20Result%20Structure%20%28by%20ref%29))
  (Utilities|Casting|CastToALS_AnimMan_CharacterBP OtherActor)
  (Rendering|SetVisibility (Variables|Default|GetInputIndicator) true false))

(event OnComponentEndOverlap(BiggerSphere)
  (params (OverlappedComponent :type Primitive%20Component%20Object%20Reference) (OtherActor :type Actor%20Object%20Reference) (OtherComp :type Primitive%20Component%20Object%20Reference) (OtherBodyIndex :type Integer))
  (Utilities|Casting|CastToALS_AnimMan_CharacterBP OtherActor)
  (Rendering|SetVisibility (Variables|Default|GetInputIndicator) false false))

(event OnComponentBeginOverlap(SmallerSphere)
  (params (OverlappedComponent :type Primitive%20Component%20Object%20Reference) (OtherActor :type Actor%20Object%20Reference) (OtherComp :type Primitive%20Component%20Object%20Reference) (OtherBodyIndex :type Integer) (bFromSweep :type Boolean) (SweepResult :type Hit%20Result%20Structure%20%28by%20ref%29))
  (Utilities|Casting|CastToALS_AnimMan_CharacterBP OtherActor)
  (Rendering|SetVisibility (Variables|Default|GetInputIndicator) false false)
  (Rendering|SetVisibility (Variables|Default|GetInput) true false)
  (Input|EnableInput (Game|GetPlayerController 0)))

(event OnComponentEndOverlap(SmallerSphere)
  (params (OverlappedComponent :type Primitive%20Component%20Object%20Reference) (OtherActor :type Actor%20Object%20Reference) (OtherComp :type Primitive%20Component%20Object%20Reference) (OtherBodyIndex :type Integer))
  (Utilities|Casting|CastToALS_AnimMan_CharacterBP OtherActor)
  (Rendering|SetVisibility (Variables|Default|GetInputIndicator) true false)
  (Rendering|SetVisibility (Variables|Default|GetInput) false false)
  (Input|DisableInput (Game|GetPlayerController 0)))

(event EventTick
  (params (DeltaSeconds :type Float%20%28single-precision%29))
  (Utilities|FlowControl|Sequence
    (:then_0
      (if (Variables|Default|GetisOnCameraMode?)
        (Rendering|SetVisibility (Variables|Default|GetPointLight) true false)
        (bind _intensity (Timeline|LighterFlickerTimeline Play)
          (:Update
            (Rendering|Components|Light|SetIntensity (Variables|Default|GetPointLight) (Math|Float|Lerp (Variables|Default|GetMinIntensity) (Variables|Default|GetMaxIntensity) _intensity))))
        (else
          (Rendering|SetVisibility (Variables|Default|GetPointLight) false false)
          (Timeline|LighterFlickerTimeline Stop))))
    (:then_1
      (if (Variables|Default|GetcanOpen?)
        (Collision|SetCollisionEnabled (Variables|Default|GetBiggerSphere) "QueryAndPhysics")
        (else
          (Collision|SetCollisionEnabled (Variables|Default|GetBiggerSphere) "NoCollision"))))))

(event Input|ActionEvents|InputActionInteract
  (params (Key :type Key%20Structure :default "None"))
  (bind _returnvalue (Game|GetPlayerController 0))
  (bind _gaveta04 (Variables|Default|GetGaveta04))
  (:Pressed
    (if (Variables|Default|GetcanOpen?)
      (Rendering|SetVisibility (Variables|Default|GetInput) false false)
      (Variables|Default|SetcanOpen? false)
      (if (not (>= (.x (Variables|/Script/Engine.SceneComponent|GetRelativeLocation (Variables|Default|GetGaveta04))) 3e+01))
        (Game|Player|SetViewTargetwithBlend (Game|GetPlayerController 0) (Components|GetOwner (Variables|Default|GetCamera)) 0.0 "VTBlend_Linear" 0.0 false)
        (Variables|Default|SetisOnCameraMode? true)
        (bind _asals_anim_man_character_bp (Utilities|Casting|CastToALS_AnimMan_CharacterBP (Game|GetPlayerCharacter 0)))
        (Input|DisableInput _asals_anim_man_character_bp (Game|GetPlayerController 0))
        (Utilities|FlowControl|Delay 1.0)
        (Audio|PlaySoundatLocation "/Game/SFX/OpeningClosingDrawer_Sound/486081__nox-sound__object-drawer-wood-open.486081__nox-sound__object-drawer-wood-open" (Transformation|GetActorLocation) "0, 0, 0" 1.0 1.0 0.0 0 0 0)
        (Components|MoveComponentTo _gaveta04 "35.000000,-39.000000,61.000000" "0,-90.000000, 0" false false 0.5 false)
        (Utilities|FlowControl|Delay 2.0)
        (bind _returnvalue_2 (Actor|GetActorOfClass "/Game/Actors_BPs/Collectible/Collectible_BP_Drawer.Collectible_BP_Drawer_C"))
        (Variables|/Game/Actors_BPs/Collectible/Collectible_BP_Drawer.Collectible_BP_Drawer_C|SetdrawerHasBeenOpened? _returnvalue_2 true)
        (Rendering|SetVisibility (Variables|Default|GetInputIndicator) true false)
        (bind _asals_anim_man_character_bp_2 (Utilities|Casting|CastToALS_AnimMan_CharacterBP (Game|GetPlayerCharacter 0)))
        (Game|Player|SetViewTargetwithBlend (Game|GetPlayerController 0) (Components|GetOwner (Variables|/Game/ThirdPersonBP/AdvancedLocomotionV4/Blueprints/CharacterLogic/ALS_AnimMan_CharacterBP.ALS_AnimMan_CharacterBP_C|GetCamera _asals_anim_man_character_bp_2)) 0.0 "VTBlend_Linear" 0.0 false)
        (Input|EnableInput _asals_anim_man_character_bp_2 _returnvalue)
        (Variables|Default|SetisOnCameraMode? false)
        (Input|DisableInput _returnvalue)
        (Collision|SetCollisionEnabled (Variables|Default|GetBiggerSphere) "NoCollision")
        (Rendering|SetVisibility (Variables|Default|GetInput) false false)
        (else
          (Components|MoveComponentTo _gaveta04 "0,-39.000000,61.000000" "0,-90.000000, 0" false false 0.5 false))))))

(fn ConstructionScript)

(fn AddtoPin
  (params (Input :type String))
  (bind _returnvalue (Game|GetPlayerController 0))
  (if (Utilities|Enum|Equal(Enum) Input (Variables|Default|GetPin))
    (Variables|Default|SetcanOpen? true)
    (Widget|RemovefromParent (Variables|Default|GetPin%20Widget%20REF))
    (Input|SetInputModeGameOnly _returnvalue)
    (Variables|/Script/Engine.PlayerController|SetbShowMouseCursor _returnvalue false)))