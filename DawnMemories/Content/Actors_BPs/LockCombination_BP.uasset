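; Interactable four-tumbler combination lock that unlocks the Drawer_BP when solved.
; Two overlap spheres drive prompts and input, and Interact flip-flops a close-up mode with lock camera, Keypad widget, cursor and timeline-flickered light.
; Tick compares the concatenated numbers of four child-actor tumblers to Combination.
; On a match, a one-shot sequence shows the drawer camera, briefly simulates physics on the lock mesh, disables the spheres and returns control.
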(event OnComponentBeginOverlap(BiggerSphere)
  (params (OverlappedComponent :type Primitive%20Component%20Object%20Reference) (OtherActor :type Actor%20Object%20Reference) (OtherComp :type Primitive%20Component%20Object%20Reference) (OtherBodyIndex :type Integer) (bFromSweep :type Boolean) (SweepResult :type Hit%20Result%20Structure%20%28by%20ref%29))
  (Utilities|Casting|CastToALS_AnimMan_CharacterBP OtherActor)
  (Rendering|SetVisibility (Variables|Default|GetInputIndicator) true false))

(event OnComponentEndOverlap(BiggerSphere)
  (params (OverlappedComponent :type Primitive%20Component%20Object%20Reference) (OtherActor :type Actor%20Object%20Reference) (OtherComp :type Primitive%20Component%20Object%20Reference) (OtherBodyIndex :type Integer))
  (Utilities|Casting|CastToALS_AnimMan_CharacterBP OtherActor)
  (Rendering|SetVisibility (Variables|Default|GetInputIndicator) false false))

(event OnComponentBeginOverlap(SmallerSphere)
  (params (OverlappedComponent :type Primitive%20Component%20Object%20Reference) (OtherActor :type Actor%20Object%20Reference) (OtherComp :type Primitive%20Component%20Object%20Reference) (OtherBodyIndex :type Integer) (bFromSweep :type Boolean) (SweepResult :type Hit%20Result%20Structure%20%28by%20ref%29))
  (Utilities|Casting|CastToALS_AnimMan_CharacterBP OtherActor)
  (Rendering|SetVisibility (Variables|Default|GetInputIndicator) false false)
  (Rendering|SetVisibility (Variables|Default|GetInput) true false)
  (Input|EnableInput (Game|GetPlayerController 0)))

(event OnComponentEndOverlap(SmallerSphere)
  (params (OverlappedComponent :type Primitive%20Component%20Object%20Reference) (OtherActor :type Actor%20Object%20Reference) (OtherComp :type Primitive%20Component%20Object%20Reference) (OtherBodyIndex :type Integer))
  (Utilities|Casting|CastToALS_AnimMan_CharacterBP OtherActor)
  (Rendering|SetVisibility (Variables|Default|GetInputIndicator) true false)
  (Rendering|SetVisibility (Variables|Default|GetInput) false false)
  (Input|DisableInput (Game|GetPlayerController 0)))

(event EventTick
  (params (DeltaSeconds :type Float%20%28single-precision%29))
  (bind _returnvalue (Game|GetPlayerController 0))
  (bind _returnvalue_2 (Game|GetPlayerController 0))
  (bind _returnvalue_3 (Game|GetPlayerController 0))
  (bind _combomatch_ (CallFunction|CheckCombination))
  (if _combomatch_
    (Utilities|FlowControl|DoOnce false
      (:Completed
        (bind _returnvalue_4 (Actor|GetActorOfClass "/Game/Actors_BPs/Drawer_BP.Drawer_BP_C"))
        (Widget|RemovefromParent (stale Input|ActionEvents|InputActionInteract _returnvalue_4))
        (Input|SetInputModeGameOnly _returnvalue)
        (Variables|/Script/Engine.PlayerController|SetbShowMouseCursor _returnvalue false)
        (Variables|/Game/Actors_BPs/Drawer_BP.Drawer_BP_C|SetcanOpen? _returnvalue_4 true)
        (Game|Player|SetViewTargetwithBlend _returnvalue_3 (Components|GetOwner (Variables|/Game/Actors_BPs/Drawer_BP.Drawer_BP_C|GetCamera _returnvalue_4)) 0.0 "VTBlend_Linear" 0.0 false)
        (Input|DisableInput (Game|GetPlayerController 0) _returnvalue_3)
        (Utilities|FlowControl|Delay 1.5)
        (Variables|Default|SetLockedState false)
        (Utilities|FlowControl|Delay 1.0)
        (Class|SkeletalMeshComponent|SetAllBodiesSimulatePhysics (Variables|Default|GetLockMesh) true)
        (Utilities|FlowControl|Delay 1.0)
        (Class|SkeletalMeshComponent|SetAllBodiesSimulatePhysics (Variables|Default|GetLockMesh) false)
        (Rendering|SetVisibility (Variables|Default|GetPointLight) false false)
        (bind _asals_anim_man_character_bp (Utilities|Casting|CastToALS_AnimMan_CharacterBP (Game|GetPlayerCharacter 0)))
        (Variables|/Game/ThirdPersonBP/AdvancedLocomotionV4/Blueprints/CharacterLogic/ALS_AnimMan_CharacterBP.ALS_AnimMan_CharacterBP_C|SetisOnInteractingMode? _asals_anim_man_character_bp false)
        (Game|Player|SetViewTargetwithBlend _returnvalue_2 (Components|GetOwner (Variables|/Game/ThirdPersonBP/AdvancedLocomotionV4/Blueprints/CharacterLogic/ALS_AnimMan_CharacterBP.ALS_AnimMan_CharacterBP_C|GetCamera _asals_anim_man_character_bp)) 0.0 "VTBlend_Linear" 0.0 false)
        (Collision|SetCollisionEnabled (Variables|Default|GetSmallerSphere) "NoCollision")
        (Input|EnableInput (Game|GetPlayerCharacter 0) _returnvalue_2)))))

(event Input|ActionEvents|InputActionInteract
  (params (Key :type Key%20Structure :default "None"))
  (bind _returnvalue (Game|GetPlayerController 0))
  (bind _returnvalue_2 (Game|GetPlayerController 0))
  (bind _returnvalue_3 (Game|GetPlayerController 0))
  (:Pressed
    (Utilities|FlowControl|FlipFlop
      (:A
        (bind _asals_anim_man_character_bp (Utilities|Casting|CastToALS_AnimMan_CharacterBP (Game|GetPlayerCharacter 0)))
        (Variables|/Game/ThirdPersonBP/AdvancedLocomotionV4/Blueprints/CharacterLogic/ALS_AnimMan_CharacterBP.ALS_AnimMan_CharacterBP_C|SetisOnInteractingMode? _asals_anim_man_character_bp true)
        (Input|DisableInput _asals_anim_man_character_bp _returnvalue)
        (Game|Player|SetViewTargetwithBlend _returnvalue (Components|GetOwner (Variables|Default|GetCamera)) 0.0 "VTBlend_Linear" 0.0 false)
        (bind _returnvalue_4 (UserInterface|CreateWidget "/Game/UI/Keypad.Keypad_C"))
        (UserInterface|Viewport|AddtoViewport _returnvalue_4 0)
        (Input|SetInputModeGameandUI _returnvalue_3 0 "DoNotLock" true)
        (Variables|/Script/Engine.PlayerController|SetbShowMouseCursor _returnvalue_3 true)
        (Rendering|SetVisibility (Variables|Default|GetInput) false false)
        (Rendering|SetVisibility (Variables|Default|GetPointLight) true false)
        (bind _intensity (Timeline|LighterFlickerTimeline Play)
          (:Update
            (Rendering|Components|Light|SetIntensity (Variables|Default|GetPointLight) (Math|Float|Lerp (Variables|Default|GetMinIntensity) (Variables|Default|GetMaxIntensity) _intensity)))))
      (:B
        (bind _asals_anim_man_character_bp_2 (Utilities|Casting|CastToALS_AnimMan_CharacterBP (Game|GetPlayerCharacter 0)))
        (Variables|/Game/ThirdPersonBP/AdvancedLocomotionV4/Blueprints/CharacterLogic/ALS_AnimMan_CharacterBP.ALS_AnimMan_CharacterBP_C|SetisOnInteractingMode? _asals_anim_man_character_bp_2 false)
        (Input|EnableInput _asals_anim_man_character_bp_2 _returnvalue_2)
        (Game|Player|SetViewTargetwithBlend _returnvalue_2 (Components|GetOwner (Variables|/Game/ThirdPersonBP/AdvancedLocomotionV4/Blueprints/CharacterLogic/ALS_AnimMan_CharacterBP.ALS_AnimMan_CharacterBP_C|GetCamera _asals_anim_man_character_bp_2)) 0.0 "VTBlend_Linear" 0.0 false)
        (Widget|RemovefromParent _returnvalue_4)
        (Input|SetInputModeGameOnly _returnvalue_3)
        (Variables|/Script/Engine.PlayerController|SetbShowMouseCursor _returnvalue_3 false)
        (Rendering|SetVisibility (Variables|Default|GetInput) true false)
        (Rendering|SetVisibility (Variables|Default|GetPointLight) false false)
        (Timeline|LighterFlickerTimeline Stop)))))

(fn ConstructionScript)

(fn CheckCombination
  (return (Utilities|Enum|Equal(Enum) (Variables|Default|GetCombination) (Utilities|String|Append (Utilities|String|ToString(Integer) (Variables|/Game/Actors_BPs/LockTumbler_BP.LockTumbler_BP_C|GetTumblerNumber (.AsLock%20Tumbler%20BP (Utilities|Casting|CastToLockTumbler_BP (Variables|/Script/Engine.ChildActorComponent|GetChildActor (Variables|Default|GetLockTumbler_BP1)))))) (Utilities|String|ToString(Integer) (Variables|/Game/Actors_BPs/LockTumbler_BP.LockTumbler_BP_C|GetTumblerNumber (.AsLock%20Tumbler%20BP (Utilities|Casting|CastToLockTumbler_BP (Variables|/Script/Engine.ChildActorComponent|GetChildActor (Variables|Default|GetLockTumbler_BP2)))))) (Utilities|String|ToString(Integer) (Variables|/Game/Actors_BPs/LockTumbler_BP.LockTumbler_BP_C|GetTumblerNumber (.AsLock%20Tumbler%20BP (Utilities|Casting|CastToLockTumbler_BP (Variables|/Script/Engine.ChildActorComponent|GetChildActor (Variables|Default|GetLockTumbler_BP3)))))) (Utilities|String|ToString(Integer) (Variables|/Game/Actors_BPs/LockTumbler_BP.LockTumbler_BP_C|GetTumblerNumber (.AsLock%20Tumbler%20BP (Utilities|Casting|CastToLockTumbler_BP (Variables|/Script/Engine.ChildActorComponent|GetChildActor (Variables|Default|GetLockTumbler_BP4))))))))))