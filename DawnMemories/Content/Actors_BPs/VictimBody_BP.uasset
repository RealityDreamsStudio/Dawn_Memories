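; VictimBody_BP is a victim body actor that the player can inspect through its own camera.
; Two nested spheres show an indicator, then an input prompt, and enable input only inside the smaller one.
; Interact toggles between this camera, with clamped mouse look and a timeline-driven flickering lighter light, and the player's camera.
; The camera raise and lower inputs call functions that currently do nothing.
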(event OnComponentBeginOverlap(BiggerSphere)
  (params (OverlappedComponent :type Primitive%20Component%20Object%20Reference) (OtherActor :type Actor%20Object%20Reference) (OtherComp :type Primitive%20Component%20Object%20Reference) (OtherBodyIndex :type Integer) (bFromSweep :type Boolean) (SweepResult :type Hit%20Result%20Structure%20%28by%20ref%29))
  (Utilities|Casting|CastToALS_AnimMan_CharacterBP OtherActor)
  (Rendering|SetVisibility (Variables|Default|GetInputIndicator) true false))

(event OnComponentEndOverlap(BiggerSphere)
  (params (OverlappedComponent :type Primitive%20Component%20Object%20Reference) (OtherActor :type Actor%20Object%20Reference) (OtherComp :type Primitive%20Component%20Object%20Reference) (OtherBodyIndex :type Integer))
  (Utilities|Casting|CastToALS_AnimMan_CharacterBP OtherActor)
  (Rendering|SetVisibility (Variables|Default|GetInputIndicator) false false)
  (Rendering|SetVisibility (Variables|Default|GetInput) false false))

(event OnComponentBeginOverlap(SmallerSphere)
  (params (OverlappedComponent :type Primitive%20Component%20Object%20Reference) (OtherActor :type Actor%20Object%20Reference) (OtherComp :type Primitive%20Component%20Object%20Reference) (OtherBodyIndex :type Integer) (bFromSweep :type Boolean) (SweepResult :type Hit%20Result%20Structure%20%28by%20ref%29))
  (Utilities|Casting|CastToALS_AnimMan_CharacterBP OtherActor)
  (Rendering|SetVisibility (Variables|Default|GetInputIndicator) false false)
  (Rendering|SetVisibility (Variables|Default|GetInput) true false)
  (Input|EnableInput (Game|GetPlayerController 0)))

(event OnComponentEndOverlap(SmallerSphere)
  (params (OverlappedComponent :type Primitive%20Component%20Object%20Reference) (OtherActor :type Actor%20Object%20Reference) (OtherComp :type Primitive%20Component%20Object%20Reference) (OtherBodyIndex :type Integer))
  (Utilities|Casting|CastToALS_AnimMan_CharacterBP OtherActor)
  (Rendering|SetVisibility (Variables|Default|GetInputIndicator) true false)
  (Rendering|SetVisibility (Variables|Default|GetInput) false false)
  (Input|DisableInput (Game|GetPlayerController 0)))

(event Collision|EventActorBeginOverlap
  (params (OtherActor :type Actor%20Object%20Reference)))

(event Input|ActionEvents|InputActionInteract
  (params (Key :type Key%20Structure :default "None"))
  (:Pressed
    (Utilities|FlowControl|FlipFlop
      (:A
        (Variables|Default|SetisOnCameraMode? true)
        (Game|Player|SetViewTargetwithBlend (Game|GetPlayerController 0) (Components|GetOwner (Variables|Default|GetCamera)) 0.0 "VTBlend_EaseInOut" 0.0 false)
        (Rendering|SetVisibility (Variables|Default|GetPointLight) true false)
        (bind _intensity (Timeline|LighterFlickerTimeline Play)
          (:Update
            (Rendering|Components|Light|SetIntensity (Variables|Default|GetPointLight) (Math|Float|Lerp (Variables|Default|GetMinIntensity) (Variables|Default|GetMaxIntensity) _intensity)))))
      (:B
        (Rendering|SetVisibility (Variables|Default|GetPointLight) false false)
        (bind _asals_anim_man_character_bp (Utilities|Casting|CastToALS_AnimMan_CharacterBP (Game|GetPlayerCharacter 0)))
        (Game|Player|SetViewTargetwithBlend (Game|GetPlayerController 0) (Components|GetOwner (Variables|/Game/ThirdPersonBP/AdvancedLocomotionV4/Blueprints/CharacterLogic/ALS_AnimMan_CharacterBP.ALS_AnimMan_CharacterBP_C|GetCamera _asals_anim_man_character_bp)) 0.0 "VTBlend_EaseInOut" 0.0 false)
        (Variables|Default|SetisOnCameraMode? false)
        (Transformation|SetRelativeRotation (Variables|Default|GetCamera) "0, 0, 0" false false)
        (Timeline|LighterFlickerTimeline Stop)))))

(event Input|ActionEvents|InputActionChangeActorCameraPositionUp
  (params (Key :type Key%20Structure :default "None"))
  (:Pressed
    (CallFunction|ElevateCamera)))

(event Input|ActionEvents|InputActionChangeActorCameraPositionDown
  (params (Key :type Key%20Structure :default "None"))
  (:Pressed
    (CallFunction|LowerCamera)))

(event Input|MouseEvents|MouseX
  (params (AxisValue :type Float%20%28single-precision%29))
  (if (Variables|Default|GetisOnCameraMode?)
    (bind _output_get (Variables|Default|SetYaw (Math|Float|Clamp(Float) (+ AxisValue (Variables|Default|GetYaw)) -5.0 5.0)))
    (Transformation|SetRelativeRotation (Variables|Default|GetCamera) (Math|Rotator|MakeRotator 0.0 (stale Input|MouseEvents|MouseY _output_get) _output_get) false false)))

(event Input|MouseEvents|MouseY
  (params (AxisValue :type Float%20%28single-precision%29))
  (if (Variables|Default|GetisOnCameraMode?)
    (bind _output_get (Variables|Default|SetPitch (Math|Float|Clamp(Float) (+ AxisValue (Variables|Default|GetPitch)) -5.0 5.0)))
    (Transformation|SetRelativeRotation (Variables|Default|GetCamera) (Math|Rotator|MakeRotator 0.0 _output_get (stale Input|MouseEvents|MouseX _output_get)) false false)))

(fn ConstructionScript)

(fn ElevateCamera
  (if (and (Variables|Default|GetisOnCameraMode?) false)
    _))

(fn LowerCamera
  (if (and (Variables|Default|GetisOnCameraMode?) false)
    _))