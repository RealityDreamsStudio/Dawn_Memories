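; Collectible key actor that the player picks up with the Interact input.
; An outer Box overlap shows an input indicator, while Box1 swaps it for the input prompt and enables input on the actor.
; Interacting updates the game mode's collectible counters, sets key flags on the ALS character including HasAllKeys once all are caught, plays a sound, destroys the actor and adds an Objectives widget.
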(event OnComponentBeginOverlap(Box)
  (params (OverlappedComponent :type Primitive%20Component%20Object%20Reference) (OtherActor :type Actor%20Object%20Reference) (OtherComp :type Primitive%20Component%20Object%20Reference) (OtherBodyIndex :type Integer) (bFromSweep :type Boolean) (SweepResult :type Hit%20Result%20Structure%20%28by%20ref%29))
  (Utilities|Casting|CastToALS_AnimMan_CharacterBP OtherActor)
  (Rendering|SetVisibility (Variables|Default|GetInputIndicator) true false))

(event OnComponentEndOverlap(Box)
  (params (OverlappedComponent :type Primitive%20Component%20Object%20Reference) (OtherActor :type Actor%20Object%20Reference) (OtherComp :type Primitive%20Component%20Object%20Reference) (OtherBodyIndex :type Integer))
  (Utilities|Casting|CastToALS_AnimMan_CharacterBP OtherActor)
  (Rendering|SetVisibility (Variables|Default|GetInputIndicator) false false))

(event OnComponentBeginOverlap(Box1)
  (params (OverlappedComponent :type Primitive%20Component%20Object%20Reference) (OtherActor :type Actor%20Object%20Reference) (OtherComp :type Primitive%20Component%20Object%20Reference) (OtherBodyIndex :type Integer) (bFromSweep :type Boolean) (SweepResult :type Hit%20Result%20Structure%20%28by%20ref%29))
  (Utilities|Casting|CastToALS_AnimMan_CharacterBP OtherActor)
  (Input|EnableInput (Game|GetPlayerController 0))
  (Rendering|SetVisibility (Variables|Default|GetInputIndicator) false false)
  (Rendering|SetVisibility (Variables|Default|GetInput) true false))

(event OnComponentEndOverlap(Box1)
  (params (OverlappedComponent :type Primitive%20Component%20Object%20Reference) (OtherActor :type Actor%20Object%20Reference) (OtherComp :type Primitive%20Component%20Object%20Reference) (OtherBodyIndex :type Integer))
  (Utilities|Casting|CastToALS_AnimMan_CharacterBP OtherActor)
  (Input|DisableInput (Game|GetPlayerController 0))
  (Rendering|SetVisibility (Variables|Default|GetInputIndicator) true false)
  (Rendering|SetVisibility (Variables|Default|GetInput) false false))

(event Collision|EventActorBeginOverlap
  (params (OtherActor :type Actor%20Object%20Reference)))

(event Input|ActionEvents|InputActionInteract
  (params (Key :type Key%20Structure))
  (bind _returnvalue (Game|GetPlayerCharacter 0))
  (:Pressed
    (bind _asals_anim_man_character_bp (Utilities|Casting|CastToALS_AnimMan_CharacterBP (Game|GetPlayerCharacter 0)))
    (Variables|/Game/ThirdPersonBP/AdvancedLocomotionV4/Blueprints/CharacterLogic/ALS_AnimMan_CharacterBP.ALS_AnimMan_CharacterBP_C|SetcaughtAKey? _asals_anim_man_character_bp true)
    (bind _asals_game_mode_sp (Utilities|Casting|CastToALS_GameMode_SP (Game|GetGameMode)))
    (bind _result (Math|Integer|DecrementInt (Variables|/Game/ThirdPersonBP/AdvancedLocomotionV4/Blueprints/GameModes/ALS_GameMode_SP.ALS_GameMode_SP_C|GetCollectibles%20Left _asals_game_mode_sp))
      (:%20%20
        (Variables|/Game/ThirdPersonBP/AdvancedLocomotionV4/Blueprints/GameModes/ALS_GameMode_SP.ALS_GameMode_SP_C|SetCollectibles%20Left _asals_game_mode_sp _result)
        (bind _result_2 (Math|Integer|IncrementInt (Variables|/Game/ThirdPersonBP/AdvancedLocomotionV4/Blueprints/GameModes/ALS_GameMode_SP.ALS_GameMode_SP_C|GetCollectiblesCaught _asals_game_mode_sp))
          (:%20%20
            (bind _output_get (Variables|/Game/ThirdPersonBP/AdvancedLocomotionV4/Blueprints/GameModes/ALS_GameMode_SP.ALS_GameMode_SP_C|SetCollectiblesCaught _asals_game_mode_sp _result_2))
            (Audio|PlaySoundatLocation "/Game/SFX/KeyPickup_Sound/512137__beezlefm__key-sound.512137__beezlefm__key-sound" (Transformation|GetActorLocation) "0, 0, 0" 1.0 1.0 0.0 0 0 0)
            (Actor|DestroyActor)
            (bind _returnvalue_2 (UserInterface|CreateWidget "/Game/UI/Objectives.Objectives_C"))
            (UserInterface|Viewport|AddtoViewport _returnvalue_2 0)
            (if (== _output_get (Variables|/Game/ThirdPersonBP/AdvancedLocomotionV4/Blueprints/GameModes/ALS_GameMode_SP.ALS_GameMode_SP_C|GetTotal%20Collectibles _asals_game_mode_sp))
              (bind _asals_anim_man_character_bp_2 (Utilities|Casting|CastToALS_AnimMan_CharacterBP _returnvalue))
              (Variables|/Game/ThirdPersonBP/AdvancedLocomotionV4/Blueprints/CharacterLogic/ALS_AnimMan_CharacterBP.ALS_AnimMan_CharacterBP_C|SethasAllKeys? _asals_anim_man_character_bp_2 true)
              (else
                (bind _asals_anim_man_character_bp_3 (Utilities|Casting|CastToALS_AnimMan_CharacterBP _returnvalue))
                (Variables|/Game/ThirdPersonBP/AdvancedLocomotionV4/Blueprints/CharacterLogic/ALS_AnimMan_CharacterBP.ALS_AnimMan_CharacterBP_C|SethasAllKeys? _asals_anim_man_character_bp_3 false)))))))))

(fn ConstructionScript)