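; Interactable bookshelf that the player inspects through its own camera, with a hidden collectible behind one book.
; Two proximity spheres drive prompts and input; Interact flip-flops camera mode, swapping view, player input, cursor, widget and flickering light.
; Up/down inputs step the spring arm through four flagged positions, which also set arrow-hiding flags.
; Hovering certain books or the frame toggles custom depth, and clicking Book_017 plays a sound and spawns the collectible.
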(event OnBeginCursorOver(simple-book-shelf_Book_003)
  (params (TouchedComponent :type Primitive%20Component%20Object%20Reference))
  ;[1 1 1] First Shelf
  (if (Variables|Default|GetisOnCameraMode?)
    (Rendering|SetRenderCustomDepth (Variables|Default|Getsimple-book-shelf_Book_003) true)))

(event OnComponentBeginOverlap(BiggerSphere)
  (params (OverlappedComponent :type Primitive%20Component%20Object%20Reference) (OtherActor :type Actor%20Object%20Reference) (OtherComp :type Primitive%20Component%20Object%20Reference) (OtherBodyIndex :type Integer) (bFromSweep :type Boolean) (SweepResult :type Hit%20Result%20Structure%20%28by%20ref%29))
  (Utilities|Casting|CastToALS_AnimMan_CharacterBP OtherActor)
  (Variables|Interaction|SetisInBiggerSphere? true)
  (Rendering|SetVisibility (Variables|Default|GetInputIndicator) true false))

(event OnEndCursorOver(simple-book-shelf_FrameGlass)
  (params (TouchedComponent :type Primitive%20Component%20Object%20Reference))
  ;[1 1 1] First Shelf
  ;;[1 1 1] Frame selection
  (Rendering|SetRenderCustomDepth (Variables|Default|Getsimple-book-shelf_Frame) false))

(event OnBeginCursorOver(simple-book-shelf_Book_013)
  (params (TouchedComponent :type Primitive%20Component%20Object%20Reference))
  ;[1 1 1] First Shelf
  (if (Variables|Default|GetisOnCameraMode?)
    (Rendering|SetRenderCustomDepth (Variables|Default|Getsimple-book-shelf_Book_013) true)))

(event OnEndCursorOver(simple-book-shelf_Book_017)
  (params (TouchedComponent :type Primitive%20Component%20Object%20Reference))
  (Rendering|SetRenderCustomDepth (Variables|Default|Getsimple-book-shelf_Book_017) false))

(event OnEndCursorOver(simple-book-shelf_Book_013)
  (params (TouchedComponent :type Primitive%20Component%20Object%20Reference))
  ;[1 1 1] First Shelf
  (Rendering|SetRenderCustomDepth (Variables|Default|Getsimple-book-shelf_Book_013) false))

(event OnClicked(simple-book-shelf_Book_017)
  (params (TouchedComponent :type Primitive%20Component%20Object%20Reference) (ButtonPressed :type Key%20Structure :default "None"))
  (Audio|PlaySoundatLocation "/Game/SFX/KeyPickup_Sound/512137__beezlefm__key-sound.512137__beezlefm__key-sound" "-409.838684,-162.644669,593.002930" "0, 0, 0" 1.0 1.0 0.0 0 0 0)
  (Game|SpawnActorfromClass "/Game/Actors_BPs/Collectible/Collectible_BP_BookShelf.Collectible_BP_BookShelf_C" (Math|Transform|MakeTransform "-409.838684,-162.644669,593.002930" "0, 0, 0" "1,1,1") "Undefined" 0 0))

(event OnComponentEndOverlap(BiggerSphere)
  (params (OverlappedComponent :type Primitive%20Component%20Object%20Reference) (OtherActor :type Actor%20Object%20Reference) (OtherComp :type Primitive%20Component%20Object%20Reference) (OtherBodyIndex :type Integer))
  (Utilities|Casting|CastToALS_AnimMan_CharacterBP OtherActor)
  (Variables|Interaction|SetisInBiggerSphere? false)
  (Rendering|SetVisibility (Variables|Default|GetInputIndicator) false false))

(event OnComponentBeginOverlap(SmallerSphere)
  (params (OverlappedComponent :type Primitive%20Component%20Object%20Reference) (OtherActor :type Actor%20Object%20Reference) (OtherComp :type Primitive%20Component%20Object%20Reference) (OtherBodyIndex :type Integer) (bFromSweep :type Boolean) (SweepResult :type Hit%20Result%20Structure%20%28by%20ref%29))
  (Utilities|Casting|CastToALS_AnimMan_CharacterBP OtherActor)
  (Variables|Interaction|SetisInSmallerSphere? true)
  (Rendering|SetVisibility (Variables|Default|GetInputIndicator) false false)
  (Rendering|SetVisibility (Variables|Default|GetInput) true false)
  (Input|EnableInput (Game|GetPlayerController 0)))

(event OnComponentEndOverlap(SmallerSphere)
  (params (OverlappedComponent :type Primitive%20Component%20Object%20Reference) (OtherActor :type Actor%20Object%20Reference) (OtherComp :type Primitive%20Component%20Object%20Reference) (OtherBodyIndex :type Integer))
  (Utilities|Casting|CastToALS_AnimMan_CharacterBP OtherActor)
  (bind _output_get (Variables|Interaction|SetisInSmallerSphere? false))
  (if (and (not _output_get) (Variables|Interaction|GetisInBiggerSphere?))
    (Rendering|SetVisibility (Variables|Default|GetInput) false false)
    (Input|DisableInput (Game|GetPlayerController 0))))

(event OnEndCursorOver(simple-book-shelf_Book_003)
  (params (TouchedComponent :type Primitive%20Component%20Object%20Reference))
  ;[1 1 1] First Shelf
  (Rendering|SetRenderCustomDepth (Variables|Default|Getsimple-book-shelf_Book_003) false))

(event OnBeginCursorOver(simple-book-shelf_Frame)
  (params (TouchedComponent :type Primitive%20Component%20Object%20Reference))
  ;[1 1 1] First Shelf
  ;;[1 1 1] Frame selection
  (if (Variables|Default|GetisOnCameraMode?)
    (Rendering|SetRenderCustomDepth (Variables|Default|Getsimple-book-shelf_Frame) true)))

(event OnEndCursorOver(simple-book-shelf_Frame)
  (params (TouchedComponent :type Primitive%20Component%20Object%20Reference))
  ;[1 1 1] First Shelf
  ;;[1 1 1] Frame selection
  (Rendering|SetRenderCustomDepth (Variables|Default|Getsimple-book-shelf_Frame) false))

(event OnBeginCursorOver(simple-book-shelf_FrameGlass)
  (params (TouchedComponent :type Primitive%20Component%20Object%20Reference))
  ;[1 1 1] First Shelf
  ;;[1 1 1] Frame selection
  (if (Variables|Default|GetisOnCameraMode?)
    (Rendering|SetRenderCustomDepth (Variables|Default|Getsimple-book-shelf_Frame) true)))

(event OnBeginCursorOver(simple-book-shelf_Book_017)
  (params (TouchedComponent :type Primitive%20Component%20Object%20Reference))
  (if (Variables|Default|GetisOnCameraMode?)
    (Rendering|SetRenderCustomDepth (Variables|Default|Getsimple-book-shelf_Book_017) true)))

(event EventTick
  (params (DeltaSeconds :type Float%20%28single-precision%29))
  (Utilities|FlowControl|Sequence
    (:then_0
      (if (Variables|Default|GetisOnPosition01?)
        (Variables|Default|SetcanHideTopArrow? true)
        (else
          (Variables|Default|SetcanHideTopArrow? false))))
    (:then_1
      (if (Variables|Default|GetisOnPosition04?)
        (Variables|Default|SetcanHideBottomArrow? true)
        (else
          (Variables|Default|SetcanHideBottomArrow? false))))))

(event Input|ActionEvents|InputActionInteract
  (params (Key :type Key%20Structure :default "None"))
  (bind _returnvalue (Game|GetPlayerController 0))
  (bind _returnvalue_2 (Game|GetPlayerController 0))
  (bind _returnvalue_3 (Game|GetPlayerController 0))
  (bind _returnvalue_4 (Game|GetPlayerController 0))
  (bind _returnvalue_5 (Game|GetPlayerCharacter 0))
  (:Pressed
    (Utilities|FlowControl|FlipFlop
      (:A
        (Rendering|SetVisibility (Variables|Default|GetInput) false false)
        (Components|Activation|Activate (Variables|Default|GetShelfCamera) false)
        (bind _asals_anim_man_character_bp (Utilities|Casting|CastToALS_AnimMan_CharacterBP (Game|GetPlayerCharacter 0)))
        (Input|DisableInput _asals_anim_man_character_bp _returnvalue_3)
        (Game|Player|SetViewTargetwithBlend _returnvalue_3 (Components|GetOwner (Variables|Default|GetShelfCamera)) 0.0 "VTBlend_Linear" 0.0 false)
        (Rendering|SetVisibility (Variables|Default|GetRectLight) true false)
        (bind _returnvalue_6 (UserInterface|CreateWidget "/Game/UI/BookShelf.BookShelf_C"))
        (UserInterface|Viewport|AddtoViewport _returnvalue_6 0)
        (Input|SetInputModeGameandUI _returnvalue_4 0 "DoNotLock" true)
        (Variables|/Script/Engine.PlayerController|SetbShowMouseCursor _returnvalue_4 true)
        (Variables|Default|SetisOnCameraMode? true)
        (Variables|Default|SetisOnPosition01? true)
        (Variables|Default|SetisOnPosition02? false)
        (Variables|Default|SetisOnPosition03? false)
        (Variables|Default|SetisOnPosition04? false)
        (bind _asals_anim_man_character_bp_2 (Utilities|Casting|CastToALS_AnimMan_CharacterBP (Game|GetPlayerCharacter 0)))
        (Variables|/Game/ThirdPersonBP/AdvancedLocomotionV4/Blueprints/CharacterLogic/ALS_AnimMan_CharacterBP.ALS_AnimMan_CharacterBP_C|SetisOnInteractingMode? _asals_anim_man_character_bp_2 true)
        (bind _intensity (Timeline|LighterFlickerTimeline Play)
          (:Update
            (Rendering|Components|Light|SetIntensity (Variables|Default|GetRectLight) (Math|Float|Lerp (Variables|Default|GetMinIntensity) (Variables|Default|GetMaxIntensity) _intensity)))))
      (:B
        (Rendering|SetVisibility (Variables|Default|GetInput) true false)
        (Rendering|SetVisibility (Variables|Default|GetRectLight) false false)
        (Components|Activation|Deactivate (Variables|Default|GetShelfCamera))
        (bind _asals_anim_man_character_bp_3 (Utilities|Casting|CastToALS_AnimMan_CharacterBP _returnvalue_5))
        (Game|Player|SetViewTargetwithBlend _returnvalue_2 (Components|GetOwner (Variables|/Game/ThirdPersonBP/AdvancedLocomotionV4/Blueprints/CharacterLogic/ALS_AnimMan_CharacterBP.ALS_AnimMan_CharacterBP_C|GetCamera _asals_anim_man_character_bp_3)) 0.0 "VTBlend_Linear" 0.0 false)
        (Input|EnableInput _returnvalue_5 _returnvalue_2)
        (Widget|RemovefromParent _returnvalue_6)
        (Input|SetInputModeGameOnly _returnvalue)
        (Variables|/Script/Engine.PlayerController|SetbShowMouseCursor _returnvalue false)
        (Variables|Default|SetisOnCameraMode? false)
        (Variables|Default|SetisOnPosition01? false)
        (Variables|Default|SetisOnPosition02? false)
        (Variables|Default|SetisOnPosition03? false)
        (Variables|Default|SetisOnPosition04? false)
        (bind _asals_anim_man_character_bp_4 (Utilities|Casting|CastToALS_AnimMan_CharacterBP (Game|GetPlayerCharacter 0)))
        (Variables|/Game/ThirdPersonBP/AdvancedLocomotionV4/Blueprints/CharacterLogic/ALS_AnimMan_CharacterBP.ALS_AnimMan_CharacterBP_C|SetisOnInteractingMode? _asals_anim_man_character_bp_4 false)
        (bind _intensity_2 (Timeline|Timeline_0 Stop)
          (:Update
            (Rendering|Components|Light|SetIntensity (Variables|Default|GetRectLight) (Math|Float|Lerp (Variables|Default|GetMinIntensity) (Variables|Default|GetMaxIntensity) _intensity_2))))))))

(event Input|ActionEvents|InputActionChangeActorCameraPositionUp
  (params (Key :type Key%20Structure :default "None"))
  (:Pressed
    (CallFunction|ElevateCamera)))

(event Input|ActionEvents|InputActionChangeActorCameraPositionDown
  (params (Key :type Key%20Structure :default "None"))
  (:Pressed
    (CallFunction|LowerCamera)))

(fn ConstructionScript)

(fn ElevateCamera
  (if (and (Variables|Default|GetisOnCameraMode?) (Variables|Default|GetisOnPosition04?))
    (Variables|/Script/Engine.SpringArmComponent|SetTargetOffset (Variables|Default|GetSpringArm) "0, 0,123.000000")
    (Variables|Default|SetisOnPosition01? false)
    (Variables|Default|SetisOnPosition02? false)
    (Variables|Default|SetisOnPosition03? true)
    (Variables|Default|SetisOnPosition04? false)
    (Variables|Default|SetcanHideTopArrow? false)
    (elif (and (Variables|Default|GetisOnCameraMode?) (Variables|Default|GetisOnPosition03?))
      (Variables|/Script/Engine.SpringArmComponent|SetTargetOffset (Variables|Default|GetSpringArm) "0, 0,173.000000")
      (Variables|Default|SetisOnPosition01? false)
      (Variables|Default|SetisOnPosition02? true)
      (Variables|Default|SetisOnPosition03? false)
      (Variables|Default|SetisOnPosition04? false)
      (Variables|Default|SetcanHideTopArrow? false)
      (elif (and (Variables|Default|GetisOnCameraMode?) (Variables|Default|GetisOnPosition02?))
        (Variables|/Script/Engine.SpringArmComponent|SetTargetOffset (Variables|Default|GetSpringArm) "0,0.000000,123.000000")
        (Variables|Default|SetisOnPosition01? true)
        (Variables|Default|SetisOnPosition02? false)
        (Variables|Default|SetisOnPosition03? false)
        (Variables|Default|SetisOnPosition04? false)
        (Variables|Default|SetcanHideTopArrow? true)))))

(fn LowerCamera
  (if (and (Variables|Default|GetisOnCameraMode?) (Variables|Default|GetisOnPosition01?))
    (Variables|/Script/Engine.SpringArmComponent|SetTargetOffset (Variables|Default|GetSpringArm) "0, 0,173.000000")
    (Variables|Default|SetisOnPosition01? false)
    (Variables|Default|SetisOnPosition02? true)
    (Variables|Default|SetisOnPosition03? false)
    (Variables|Default|SetcanHideBottomArrow? false)
    (Variables|Default|SetcanHideBottomArrow? false)
    (elif (and (Variables|Default|GetisOnCameraMode?) (Variables|Default|GetisOnPosition02?))
      (Variables|/Script/Engine.SpringArmComponent|SetTargetOffset (Variables|Default|GetSpringArm) "0, 0,123.000000")
      (Variables|Default|SetisOnPosition01? false)
      (Variables|Default|SetisOnPosition02? false)
      (Variables|Default|SetisOnPosition03? true)
      (Variables|Default|SetisOnPosition04? false)
      (Variables|Default|SetcanHideBottomArrow? false)
      (elif (and (Variables|Default|GetisOnCameraMode?) (Variables|Default|GetisOnPosition03?))
        (Variables|/Script/Engine.SpringArmComponent|SetTargetOffset (Variables|Default|GetSpringArm) "0, 0,73.000000")
        (Variables|Default|SetisOnPosition01? false)
        (Variables|Default|SetisOnPosition02? false)
        (Variables|Default|SetisOnPosition03? false)
        (Variables|Default|SetisOnPosition04? true)
        (Variables|Default|SetcanHideBottomArrow? true)))))