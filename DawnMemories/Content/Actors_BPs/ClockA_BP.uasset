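; Interactive clock puzzle actor whose hands the player turns to a target time.
; Two overlap volumes stage prompts and input; Interact toggles a clock camera view with a flickering light, suspending character input.
; While viewing, Tick rotates the hour hand, geared minute hand and time-scaled seconds hand from held input.
; Tick also sets IsClockARight when all pitches are within tolerance, clearing the rotation flags; real-time clock code is unconnected.
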(event OnComponentBeginOverlap(SmallerSphere)
  (params (OverlappedComponent :type Primitive%20Component%20Object%20Reference) (OtherActor :type Actor%20Object%20Reference) (OtherComp :type Primitive%20Component%20Object%20Reference) (OtherBodyIndex :type Integer) (bFromSweep :type Boolean) (SweepResult :type Hit%20Result%20Structure%20%28by%20ref%29))
  (Utilities|Casting|CastToALS_AnimMan_CharacterBP OtherActor)
  (Rendering|SetVisibility (Variables|Default|GetInputIndicator) false false)
  (Rendering|SetVisibility (Variables|Default|GetInput) true false)
  (Input|EnableInput (Game|GetPlayerController 0)))

(event OnComponentEndOverlap(SmallerSphere)
  (params (OverlappedComponent :type Primitive%20Component%20Object%20Reference) (OtherActor :type Actor%20Object%20Reference) (OtherComp :type Primitive%20Component%20Object%20Reference) (OtherBodyIndex :type Integer))
  (Utilities|Casting|CastToALS_AnimMan_CharacterBP OtherActor)
  (Rendering|SetVisibility (Variables|Default|GetInputIndicator) true false)
  (Rendering|SetVisibility (Variables|Default|GetInput) false false)
  (Input|DisableInput (Game|GetPlayerController 0)))

(event OnComponentBeginOverlap(BiggerBox)
  (params (OverlappedComponent :type Primitive%20Component%20Object%20Reference) (OtherActor :type Actor%20Object%20Reference) (OtherComp :type Primitive%20Component%20Object%20Reference) (OtherBodyIndex :type Integer) (bFromSweep :type Boolean) (SweepResult :type Hit%20Result%20Structure%20%28by%20ref%29))
  (Utilities|Casting|CastToALS_AnimMan_CharacterBP OtherActor)
  (Rendering|SetVisibility (Variables|Default|GetInputIndicator) true false))

(event OnComponentEndOverlap(BiggerBox)
  (params (OverlappedComponent :type Primitive%20Component%20Object%20Reference) (OtherActor :type Actor%20Object%20Reference) (OtherComp :type Primitive%20Component%20Object%20Reference) (OtherBodyIndex :type Integer))
  (Utilities|Casting|CastToALS_AnimMan_CharacterBP OtherActor)
  (Rendering|SetVisibility (Variables|Default|GetInputIndicator) false false)
  (Rendering|SetVisibility (Variables|Default|GetInput) false false))

(event EventTick
  (params (DeltaSeconds :type Float%20%28single-precision%29))
  (bind _step (Variables|Default|Getstep))
  (bind _returnvalue (* _step 1.0))
  (bind _returnvalue_2 (* _step -1.0))
  (Utilities|FlowControl|Sequence
    (:then_0
      (if (and (Variables|Default|GetcanChangeClockHandRotationToTheRight?) (Variables|Default|GetisOnCameraMode?))
        (Transformation|AddLocalRotation (Variables|Default|GetClock_Hour_Hand) (Math|Rotator|MakeRotator 0.0 _returnvalue_2 0.0) false false)
        (Transformation|AddLocalRotation (Variables|Default|GetClock_Minutes_Hand) (Math|Rotator|MakeRotator 0.0 (* _returnvalue_2 12.0) 0.0) false false)
        (Transformation|AddLocalRotation (Variables|Default|GetClock_Seconds_Hand) (Math|Rotator|MakeRotator 0.0 (* (* (Variables|Default|GetClock) -3.0) (Variables|Default|Getstep)) 0.0) false false)
        (elif (and (Variables|Default|GetisOnCameraMode?) (Variables|Default|GetcanChangeClockHandRotationToTheLeft?))
          (Transformation|AddLocalRotation (Variables|Default|GetClock_Hour_Hand) (Math|Rotator|MakeRotator 0.0 _returnvalue 0.0) false false)
          (Transformation|AddLocalRotation (Variables|Default|GetClock_Minutes_Hand) (Math|Rotator|MakeRotator 0.0 (* _returnvalue 12.0) 0.0) false false)
          (Transformation|AddLocalRotation (Variables|Default|GetClock_Seconds_Hand) (Math|Rotator|MakeRotator 0.0 (* (* (Variables|Default|GetClock) 3.0) (Variables|Default|Getstep)) 0.0) false false))))
    (:then_1
      (Variables|Default|SetClock (+ (Variables|Default|GetClock) DeltaSeconds)))
    (:then_3
      (if (Math|Boolean|ANDBoolean (Math|Rotator|Equal(Rotator) (Math|Rotator|MakeRotator 0.0 (.pitch (.rotation (Transformation|GetRelativeTransform (Variables|Default|GetClock_Hour_Hand)))) 0.0) "30.000000, 0, 0" 2e+01) (Math|Rotator|Equal(Rotator) (Math|Rotator|MakeRotator 0.0 (.pitch (.rotation (Transformation|GetRelativeTransform (Variables|Default|GetClock_Minutes_Hand)))) 0.0) "7.000000, 0, 0" 2e+01) (Math|Rotator|Equal(Rotator) (Math|Rotator|MakeRotator 0.0 (.pitch (.rotation (Transformation|GetRelativeTransform (Variables|Default|GetClock_Seconds_Hand)))) 0.0) "-70.000000, 0, 0" 2e+01))
        (Variables|Default|SetisClockA%20Right? true)
        (Variables|Default|SetcanChangeClockHandRotationToTheRight? false)
        (Variables|Default|SetcanChangeClockHandRotationToTheLeft? false)
        (else
          (Variables|Default|SetisClockA%20Right? false))))))

(event Input|ActionEvents|InputActionInteract
  (params (Key :type Key%20Structure :default "None"))
  (bind _returnvalue (Game|GetPlayerController 0))
  (bind _returnvalue_2 (Game|GetPlayerController 0))
  (bind _returnvalue_3 (Game|GetPlayerCharacter 0))
  (:Pressed
    (Utilities|FlowControl|FlipFlop
      (:A
        (Input|DisableInput (Game|GetPlayerCharacter 0) _returnvalue_2)
        (Game|Player|SetViewTargetwithBlend _returnvalue_2 (Components|GetOwner (Variables|Default|GetCamera)) 0.0 "VTBlend_Linear" 0.0 false)
        (Rendering|SetVisibility (Variables|Default|GetInput) false false)
        (Variables|Default|SetisOnCameraMode? true)
        (bind _asals_anim_man_character_bp (Utilities|Casting|CastToALS_AnimMan_CharacterBP (Game|GetPlayerCharacter 0)))
        (Variables|/Game/ThirdPersonBP/AdvancedLocomotionV4/Blueprints/CharacterLogic/ALS_AnimMan_CharacterBP.ALS_AnimMan_CharacterBP_C|SetisOnInteractingMode? _asals_anim_man_character_bp true)
        (Rendering|SetVisibility (Variables|Default|GetPointLight) true false)
        (bind _intensity (Timeline|LighterFlickerTimeline Play)
          (:Update
            (Rendering|Components|Light|SetIntensity (Variables|Default|GetPointLight) (Math|Float|Lerp (Variables|Default|GetMinIntensity) (Variables|Default|GetMaxIntensity) _intensity)))))
      (:B
        (if (Variables|Default|GetisOnCameraMode?)
          (bind _asals_anim_man_character_bp_2 (Utilities|Casting|CastToALS_AnimMan_CharacterBP _returnvalue_3))
          (Game|Player|SetViewTargetwithBlend _returnvalue (Components|GetOwner (Variables|/Game/ThirdPersonBP/AdvancedLocomotionV4/Blueprints/CharacterLogic/ALS_AnimMan_CharacterBP.ALS_AnimMan_CharacterBP_C|GetCamera _asals_anim_man_character_bp_2)) 0.0 "VTBlend_Linear" 0.0 false)
          (Input|EnableInput _returnvalue_3 _returnvalue)
          (Rendering|SetVisibility (Variables|Default|GetInput) true false)
          (Variables|Default|SetisOnCameraMode? false)
          (bind _asals_anim_man_character_bp_3 (Utilities|Casting|CastToALS_AnimMan_CharacterBP (Game|GetPlayerCharacter 0)))
          (Variables|/Game/ThirdPersonBP/AdvancedLocomotionV4/Blueprints/CharacterLogic/ALS_AnimMan_CharacterBP.ALS_AnimMan_CharacterBP_C|SetisOnInteractingMode? _asals_anim_man_character_bp_3 false)
          (Rendering|SetVisibility (Variables|Default|GetPointLight) false false)
          (bind _intensity_2 (Timeline|Timeline_0 Stop)
            (:Update
              (Rendering|Components|Light|SetIntensity (Variables|Default|GetPointLight) (Math|Float|Lerp (Variables|Default|GetMinIntensity) (Variables|Default|GetMaxIntensity) _intensity_2)))))))))

(event Input|ActionEvents|InputActionRotateClockHandToTheRight
  (params (Key :type Key%20Structure :default "None"))
  (:Pressed
    (Variables|Default|SetcanChangeClockHandRotationToTheLeft? true))
  (:Released
    (Variables|Default|SetcanChangeClockHandRotationToTheLeft? false)))

(event Input|ActionEvents|InputActionRotateClockHandToTheLeft
  (params (Key :type Key%20Structure :default "None"))
  (:Pressed
    (Variables|Default|SetcanChangeClockHandRotationToTheRight? true))
  (:Released
    (Variables|Default|SetcanChangeClockHandRotationToTheRight? false)))

(fn ConstructionScript)