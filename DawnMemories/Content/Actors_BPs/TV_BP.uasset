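; TV actor that plays a static video and noise in a scripted cutaway, then a reversed puzzle voice clip.
; PlayTVStaticVideo, not called within this Blueprint, swaps the glass material for a MediaPlayer video material and turns on a spotlight.
; Timed delays disable player input, blend the view to the TV and back to the ALS character, then play the voice.
; The sphere overlap only casts to the character.
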(event OnComponentBeginOverlap(Sphere)
  (params (OverlappedComponent :type Primitive%20Component%20Object%20Reference) (OtherActor :type Actor%20Object%20Reference) (OtherComp :type Primitive%20Component%20Object%20Reference) (OtherBodyIndex :type Integer) (bFromSweep :type Boolean) (SweepResult :type Hit%20Result%20Structure%20%28by%20ref%29))
  (Utilities|Casting|CastToALS_AnimMan_CharacterBP OtherActor))

(event Custom|Play%20TV%20Static%20Video
  (bind _returnvalue (Game|GetPlayerController 0))
  (bind _returnvalue_2 (Game|GetPlayerController 0))
  (bind _media_player (Variables|Default|GetMedia%20Player))
  (Rendering|Material|SetMaterial (Variables|Default|GetStaticMesh) 1 "/Game/Movies/TV_MediaPlayer_Video_Mat.TV_MediaPlayer_Video_Mat")
  (Media|MediaPlayer|OpenSource _media_player "/Game/Movies/TV_Static_HD_Video_720P_HD.TV_Static_HD_Video_720P_HD")
  (Media|MediaPlayer|Play _media_player :!class /Script/MediaAssets.MediaPlayer)
  (Rendering|SetVisibility (Variables|Default|GetSpotLight) true false)
  (Audio|PlaySoundatLocation "/Game/SFX/TV-static-noise-HD-1080p_160k_Cue.TV-static-noise-HD-1080p_160k_Cue" (Transformation|GetActorLocation) "0, 0, 0" 1.0 1.0 0.0 "/Game/SFX/TV_StaticNoise_SoundAttenuation.TV_StaticNoise_SoundAttenuation" 0 0)
  (Input|DisableInput (Game|GetPlayerCharacter 0) _returnvalue)
  (Utilities|FlowControl|Delay 3.0)
  (Game|Player|SetViewTargetwithBlend _returnvalue (Components|GetOwner (Variables|Default|GetCamera)) 0.0 "VTBlend_Linear" 0.0 false)
  (Utilities|FlowControl|Delay 3.0)
  (bind _asals_anim_man_character_bp (Utilities|Casting|CastToALS_AnimMan_CharacterBP (Game|GetPlayerCharacter 0)))
  (Game|Player|SetViewTargetwithBlend _returnvalue_2 (Components|GetOwner (Variables|/Game/ThirdPersonBP/AdvancedLocomotionV4/Blueprints/CharacterLogic/ALS_AnimMan_CharacterBP.ALS_AnimMan_CharacterBP_C|GetCamera _asals_anim_man_character_bp)) 0.0 "VTBlend_Linear" 0.0 false)
  (Input|EnableInput _asals_anim_man_character_bp _returnvalue_2)
  (Utilities|FlowControl|Delay 3.0)
  (bind _returnvalue_3 (Audio|SpawnSoundatLocation "/Game/SFX/Character_VO/testeVozPuzzleTV_Insert6_Reverse.testeVozPuzzleTV_Insert6_Reverse" (Transformation|GetActorLocation) "0, 0, 0" 1.0 1.0 0.0 "/Game/SFX/TV_StaticNoise_SoundAttenuation.TV_StaticNoise_SoundAttenuation" 0))
  (Variables|Default|SetaudioTVREV _returnvalue_3))

(event EventBeginPlay
  (Rendering|Material|SetMaterial (Variables|Default|GetStaticMesh) 1 "/Game/WorldAssets/TV/tv_glass.tv_glass"))

(fn ConstructionScript)