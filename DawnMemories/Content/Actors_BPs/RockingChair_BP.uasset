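; Rocking chair actor that animates a back-and-forth rocking motion with a chair squeak sound.
; While CanMove is true, Tick plays a timeline whose two tracks drive lerps of the Cube's relative Y location and roll between back and forth limits.
; The timeline update also passes through a DoOnce with no visible reset, so the squeak fires at the actor's location only once.
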(event Collision|EventActorBeginOverlap
  (params (OtherActor :type Actor%20Object%20Reference)))

(event EventTick
  (params (DeltaSeconds :type Float%20%28single-precision%29))
  (if (Variables|Default|GetcanMove?)
    (bind (_direction _back_forth_location _back_forth_rotation) (Timeline|Timeline_0 Play)
      (:Update
        (Transformation|SetRelativeLocationAndRotation (Variables|Default|GetCube) (Math|Vector|MakeVector 0.0 (Math|Float|Lerp (Variables|Default|GetBack%20Loc) (Variables|Default|GetForth%20Loc) _back_forth_location) 0.0) (Math|Rotator|MakeRotator (Math|Float|Lerp (Variables|Default|GetBack%20Angle) (Variables|Default|GetForth%20Angle) _back_forth_rotation) 0.0 0.0) false false)
        (Utilities|FlowControl|DoOnce false
          (:Completed
            (Audio|PlaySoundatLocation "/Game/SFX/RockingChair_Sound/71827__sacredmatt__chair-squeak_Cue.71827__sacredmatt__chair-squeak_Cue" (Transformation|GetActorLocation) "0, 0, 0" 1.0 1.0 0.0 0 0 0)))))))

(fn ConstructionScript)