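; Interactable VHS player that plays a tape-insertion cutscene if the player character has the VHS tape.
; Two overlap spheres drive indicator and input-prompt visibility on Tick, with the inner one enabling Interact.
; Interact blends to its camera, then either animates insertion, swaps TV_BP audio and stays disabled, or briefly shows a VHS widget and allows retrying.
; Inventory-based tape selection is left unwired.
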(event OnComponentBeginOverlap(BiggerSphere)
  (params (OverlappedComponent :type Primitive%20Component%20Object%20Reference) (OtherActor :type Actor%20Object%20Reference) (OtherComp :type Primitive%20Component%20Object%20Reference) (OtherBodyIndex :type Integer) (bFromSweep :type Boolean) (SweepResult :type Hit%20Result%20Structure%20%28by%20ref%29))
  (Utilities|Casting|CastToALS_AnimMan_CharacterBP OtherActor)
  (Variables|Default|SetisInBiggerSphere? true))

(event OnComponentEndOverlap(BiggerSphere)
  (params (OverlappedComponent :type Primitive%20Component%20Object%20Reference) (OtherActor :type Actor%20Object%20Reference) (OtherComp :type Primitive%20Component%20Object%20Reference) (OtherBodyIndex :type Integer))
  (Utilities|Casting|CastToALS_AnimMan_CharacterBP OtherActor)
  (Variables|Default|SetisInBiggerSphere? false))

(event OnComponentBeginOverlap(SmallerSphere)
  (params (OverlappedComponent :type Primitive%20Component%20Object%20Reference) (OtherActor :type Actor%20Object%20Reference) (OtherComp :type Primitive%20Component%20Object%20Reference) (OtherBodyIndex :type Integer) (bFromSweep :type Boolean) (SweepResult :type Hit%20Result%20Structure%20%28by%20ref%29))
  (Utilities|Casting|CastToALS_AnimMan_CharacterBP OtherActor)
  (Variables|Default|SetisInSmallerSphere? true)
  (Input|EnableInput (Game|GetPlayerController 0)))

(event OnComponentEndOverlap(SmallerSphere)
  (params (OverlappedComponent :type Primitive%20Component%20Object%20Reference) (OtherActor :type Actor%20Object%20Reference) (OtherComp :type Primitive%20Component%20Object%20Reference) (OtherBodyIndex :type Integer))
  (Utilities|Casting|CastToALS_AnimMan_CharacterBP OtherActor)
  (Variables|Default|SetisInSmallerSphere? false)
  (Input|DisableInput (Game|GetPlayerController 0)))

(event EventTick
  (params (DeltaSeconds :type Float%20%28single-precision%29))
  (if (and (Variables|Default|GetisInBiggerSphere?) (Variables|Default|GetisInSmallerSphere?))
    (Rendering|SetVisibility (Variables|Default|GetInputIndicator) false false)
    (Rendering|SetVisibility (Variables|Default|GetInput) true false)
    (elif (Variables|Default|GetisInBiggerSphere?)
      (if (Variables|Default|GetisInSmallerSphere?)
        (if (Variables|Default|GetisOnCameraMode?)
          _)
        (else
          (Rendering|SetVisibility (Variables|Default|GetInputIndicator) true false)
          (Rendering|SetVisibility (Variables|Default|GetInput) false false)))
      (else
        (Rendering|SetVisibility (Variables|Default|GetInputIndicator) false false)))))

(event Input|ActionEvents|InputActionInteract
  (params (Key :type Key%20Structure :default "None"))
  (bind _returnvalue (Game|GetPlayerController 0))
  (bind _returnvalue_2 (Game|GetPlayerController 0))
  (bind _returnvalue_3 (Game|GetPlayerCharacter 0))
  (bind _returnvalue_4 (Game|GetPlayerController 0))
  (bind _returnvalue_5 (Game|GetPlayerCharacter 0))
  (bind _skeletalmesh1 (Variables|Default|GetSkeletalMesh1))
  (:Pressed
    (bind _asals_anim_man_character_bp (Utilities|Casting|CastToALS_AnimMan_CharacterBP (Game|GetPlayerCharacter 0)))
    (if (Variables|/Game/ThirdPersonBP/AdvancedLocomotionV4/Blueprints/CharacterLogic/ALS_AnimMan_CharacterBP.ALS_AnimMan_CharacterBP_C|GethasVHSTape? _asals_anim_man_character_bp)
      (Variables|Default|SetcanUseVHSTape? true)
      (Input|DisableInput _returnvalue)
      (Input|DisableInput (Game|GetPlayerCharacter 0) _returnvalue)
      (Variables|Default|SetisOnCameraMode? true)
      (bind _asals_anim_man_character_bp_2 (Utilities|Casting|CastToALS_AnimMan_CharacterBP (Game|GetPlayerCharacter 0)))
      (Variables|/Game/ThirdPersonBP/AdvancedLocomotionV4/Blueprints/CharacterLogic/ALS_AnimMan_CharacterBP.ALS_AnimMan_CharacterBP_C|SetisOnInteractingMode? _asals_anim_man_character_bp_2 true)
      (Game|Player|SetViewTargetwithBlend (Game|GetPlayerController 0) (Components|GetOwner (Variables|Default|GetCamera)) 0.0 "VTBlend_EaseInOut" 0.0 false)
      (Audio|PlaySoundatLocation "/Game/SFX/VHS_Sound/216766__panzen__59-vhs-casette-in_Cue.216766__panzen__59-vhs-casette-in_Cue" (Transformation|GetActorLocation) "0, 0, 0" 1.0 1.0 0.0 0 0 0)
      (Rendering|SetVisibility _skeletalmesh1 true false)
      (Audio|Components|Audio|Play _skeletalmesh1 false)
      (Audio|Components|Audio|Play (Variables|Default|GetSkeletalMesh) false)
      (bind _returnvalue_6 (Actor|GetActorOfClass "/Game/Actors_BPs/TV_BP.TV_BP_C"))
      (Audio|Components|Audio|Stop (Variables|/Game/Actors_BPs/TV_BP.TV_BP_C|GetaudioTVREV _returnvalue_6))
      (Utilities|FlowControl|Delay 5.0)
      (bind _asals_anim_man_character_bp_3 (Utilities|Casting|CastToALS_AnimMan_CharacterBP (Game|GetPlayerCharacter 0)))
      (Game|Player|SetViewTargetwithBlend (Game|GetPlayerController 0) (Components|GetOwner (Variables|/Game/ThirdPersonBP/AdvancedLocomotionV4/Blueprints/CharacterLogic/ALS_AnimMan_CharacterBP.ALS_AnimMan_CharacterBP_C|GetCamera _asals_anim_man_character_bp_3)) 0.0 "VTBlend_EaseInOut" 0.0 false)
      (Variables|Default|SetisOnCameraMode? false)
      (Collision|SetCollisionEnabled (Variables|Default|GetSmallerSphere) "NoCollision")
      (bind _asals_anim_man_character_bp_4 (Utilities|Casting|CastToALS_AnimMan_CharacterBP _returnvalue_5))
      (Variables|/Game/ThirdPersonBP/AdvancedLocomotionV4/Blueprints/CharacterLogic/ALS_AnimMan_CharacterBP.ALS_AnimMan_CharacterBP_C|SetisOnInteractingMode? _asals_anim_man_character_bp_4 false)
      (Input|EnableInput _returnvalue_5 (Game|GetPlayerController 0))
      (bind _returnvalue_7 (Actor|GetActorOfClass "/Game/Actors_BPs/TV_BP.TV_BP_C"))
      (Audio|SpawnSoundatLocation "/Game/SFX/Character_VO/words_audio.words_audio" (Transformation|GetActorLocation _returnvalue_7) "0, 0, 0" 1.0 1.0 0.0 "/Game/SFX/TV_StaticNoise_SoundAttenuation.TV_StaticNoise_SoundAttenuation" 0)
      (else
        (Variables|Default|SetcanUseVHSTape? false)
        (Input|DisableInput _returnvalue_2)
        (Input|DisableInput (Game|GetPlayerCharacter 0) _returnvalue_2)
        (Variables|Default|SetisOnCameraMode? true)
        (bind _asals_anim_man_character_bp_5 (Utilities|Casting|CastToALS_AnimMan_CharacterBP (Game|GetPlayerCharacter 0)))
        (Variables|/Game/ThirdPersonBP/AdvancedLocomotionV4/Blueprints/CharacterLogic/ALS_AnimMan_CharacterBP.ALS_AnimMan_CharacterBP_C|SetisOnInteractingMode? _asals_anim_man_character_bp_5 true)
        (Game|Player|SetViewTargetwithBlend (Game|GetPlayerController 0) (Components|GetOwner (Variables|Default|GetCamera)) 0.0 "VTBlend_EaseInOut" 0.0 false)
        (bind _returnvalue_8 (UserInterface|CreateWidget "/Game/UI/VHS.VHS_C"))
        (UserInterface|Viewport|AddtoViewport _returnvalue_8 0)
        (Collision|SetCollisionEnabled (Variables|Default|GetSmallerSphere) "NoCollision")
        (Utilities|FlowControl|Delay 3.0)
        (Widget|RemovefromParent _returnvalue_8)
        (bind _asals_anim_man_character_bp_6 (Utilities|Casting|CastToALS_AnimMan_CharacterBP (Game|GetPlayerCharacter 0)))
        (Game|Player|SetViewTargetwithBlend (Game|GetPlayerController 0) (Components|GetOwner (Variables|/Game/ThirdPersonBP/AdvancedLocomotionV4/Blueprints/CharacterLogic/ALS_AnimMan_CharacterBP.ALS_AnimMan_CharacterBP_C|GetCamera _asals_anim_man_character_bp_6)) 0.0 "VTBlend_EaseInOut" 0.0 false)
        (Variables|Default|SetisOnCameraMode? false)
        (Collision|SetCollisionEnabled (Variables|Default|GetSmallerSphere) "QueryAndPhysics")
        (bind _asals_anim_man_character_bp_7 (Utilities|Casting|CastToALS_AnimMan_CharacterBP _returnvalue_3))
        (Variables|/Game/ThirdPersonBP/AdvancedLocomotionV4/Blueprints/CharacterLogic/ALS_AnimMan_CharacterBP.ALS_AnimMan_CharacterBP_C|SetisOnInteractingMode? _asals_anim_man_character_bp_7 false)
        (Input|EnableInput _returnvalue_3 _returnvalue_4)
        (Input|EnableInput _returnvalue_4)))))

(fn ConstructionScript)