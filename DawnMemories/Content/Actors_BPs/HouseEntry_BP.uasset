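; HouseEntry_BP is a one-shot trigger actor, named for a house entry, that plays an audio cue and narration when the player character type overlaps its box.
; The overlap starts a 2D darkness sound, then after a delay plays the game-start voice line at the player's location with a Subtitles widget on screen.
; Chained delays time the sequence, removing the subtitles and then destroying the actor.
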(event OnComponentBeginOverlap(Box)
  (params (OverlappedComponent :type Primitive%20Component%20Object%20Reference) (OtherActor :type Actor%20Object%20Reference) (OtherComp :type Primitive%20Component%20Object%20Reference) (OtherBodyIndex :type Integer) (bFromSweep :type Boolean) (SweepResult :type Hit%20Result%20Structure%20%28by%20ref%29))
  (Utilities|Casting|CastToALS_AnimMan_CharacterBP OtherActor)
  (Audio|SpawnSound2D "/Game/SFX/557567__wandersound__darkness-02.557567__wandersound__darkness-02" 1.0 1.0 0.0 0)
  (Utilities|FlowControl|Delay 6.0)
  (bind _asals_anim_man_character_bp (Utilities|Casting|CastToALS_AnimMan_CharacterBP (Game|GetPlayerCharacter 0)))
  (Audio|PlaySoundatLocation "/Game/SFX/Character_VO/VO_GameStart_01.VO_GameStart_01" (Transformation|GetActorLocation _asals_anim_man_character_bp) "0, 0, 0" 1.0 1.0 0.0 0 0 0)
  (bind _returnvalue (UserInterface|CreateWidget "/Game/UI/Subtitles.Subtitles_C"))
  (UserInterface|Viewport|AddtoViewport _returnvalue 0)
  (Utilities|FlowControl|Delay 3.0)
  (Widget|RemovefromParent _returnvalue)
  (Utilities|FlowControl|Delay 1.0)
  (Actor|DestroyActor))

(fn ConstructionScript)